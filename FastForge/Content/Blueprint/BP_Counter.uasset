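; Interactable counter where the player places orderable inventory items or takes the placed one back.
; Its widget button, gated on sphere overlap, moves items through player controller messages, updating the mesh from ItemTable and a red/green occupancy material.
; OnObjectPlaced fires after a short random delay, and RemoveObject can also clear the counter without returning the item.
; A construction-script trace snaps the Plane marker to the ground as MovePlayerTo's offset target.
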(event Custom|AddItem
  (bind _controller (Class|IGamemode|GetPlayerController(Message) (Game|GetGameMode)))
  (if (Collision|IsOverlappingActor (Variables|Default|GetSphere) (Pawn|GetControlledPawn _controller) :!class /Script/Engine.PrimitiveComponent)
    (if (not (Variables|Default|GetItemPlaced))
      (bind _items (Class|IController|GetInventory(Message) _controller))
      (for _array_element _items
        (bind _returnvalue (Utilities|GetDataTableRow (Variables|Default|GetItemTable) (Utilities|String|StringToName _array_element))
          (:then
            (if (> (Utilities|Struct|BreaksItemData _returnvalue) 0.0)
              (CallFunction|PlaceObject _array_element _returnvalue)))))
      (else
        (CallFunction|RemoveObject true)))))

(event Custom|MovePlayerTo
  (bind _controller (Class|IGamemode|GetPlayerController(Message) (Game|GetGameMode)))
  (bind _outlocation (CallFunction|ApplyRadialOffset (Pawn|GetControlledPawn _controller) (Transformation|GetWorldLocation (Variables|Default|GetPlane)) 25.0))
  (Class|IController|TryCharacterMove(Message) _controller _outlocation))

(event Custom|PlaceObject
  (params (ID :type String) (Data :type S%20Item%20Data%20Structure))
  (bind _controller (Class|IGamemode|GetPlayerController(Message) (Game|GetGameMode)))
  (bind _success (Class|IController|RemoveItem(Message) _controller ID))
  (if _success
    (bind _output_get (Variables|Default|SetStoredID ID))
    (Variables|Default|SetItemPlaced true)
    (Rendering|Material|SetMaterial (Variables|Default|GetCube1) 0 "/Game/Blueprint/M_Green.M_Green")
    (bind _returnvalue (Utilities|GetDataTableRow (Variables|Default|GetItemTable) (Utilities|String|StringToName _output_get))
      (:then
        (Components|StaticMesh|SetStaticMesh (Variables|Default|GetItem) (.ItemMesh (Utilities|Struct|BreaksItemData _returnvalue)))
        (Utilities|IsValid (.ItemMeshMaterial (Utilities|Struct|BreaksItemData _returnvalue))
          (:Is%20Valid
            (Rendering|Material|SetMaterial (Variables|Default|GetItem) 0 (.ItemMeshMaterial (Utilities|Struct|BreaksItemData _returnvalue))))
          (:Is%20Not%20Valid
            _)))
      (:RowNotFound
        (Components|StaticMesh|SetStaticMesh (Variables|Default|GetItem) 0)))
    (Utilities|FlowControl|Delay (Math|Random|RandomFloatinRange 0.5 2.0))
    (Default|CallOnObjectPlaced (Variables|Default|GetStoredID) self)))

(event Custom|RemoveObject
  (params (ReturnToPlayer :type Boolean))
  (if ReturnToPlayer
    (bind _controller (Class|IGamemode|GetPlayerController(Message) (Game|GetGameMode)))
    (bind _success (Class|IController|GiveItem(Message) _controller (Variables|Default|GetStoredID)))
    (Variables|Default|SetItemPlaced (not _success))
    (else
      (Variables|Default|SetItemPlaced false)))
  (Variables|Default|SetStoredID "")
  (Rendering|Material|SetMaterial (Variables|Default|GetCube1) 0 "/Game/Blueprint/M_Red.M_Red")
  (Components|StaticMesh|SetStaticMesh (Variables|Default|GetItem) 0))

(event EventBeginPlay
  (bind _returnvalue (UserInterface|CreateWidget "/Game/Blueprint/UI/UI_StandardButton.UI_StandardButton_C"))
  (UserInterface|SetWidget (Variables|Default|GetWidget) _returnvalue)
  (EventDispatchers|BindEventtoOnButtonClicked _returnvalue (delegate Custom|AddItem))
  (EventDispatchers|BindEventtoOnButtonHovered _returnvalue (EventDispatchers|CreateEvent :!event Custom|MovePlayerTo)))

(fn ConstructionScript
  (bind _returnvalue (Transformation|GetActorLocation))
  (bind _plane (Variables|Default|GetPlane))
  (bind _returnvalue_2 (Transformation|GetWorldLocation _plane))
  (bind _returnvalue_3 (Math|Vector|MakeVector (.x _returnvalue_2) (.y _returnvalue_2) (.z _returnvalue)))
  (bind (_outhit _returnvalue_4) (Collision|LineTraceByChannel _returnvalue_3 (- _returnvalue_3 "0, 0,200.000000") "TraceTypeQuery1" false 0 "ForDuration"))
  (if _returnvalue_4
    (Transformation|SetWorldLocation (Variables|Default|GetPlane) (+ (.Location (Collision|BreakHitResult _outhit)) "0, 0,1.000000") false false)))

(fn ShowPlayerLocation
  (params (bNewVisibility :type Boolean))
  (Rendering|SetVisibility (Variables|Default|GetPlane) bNewVisibility false))