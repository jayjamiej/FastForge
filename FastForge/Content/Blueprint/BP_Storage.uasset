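; BP_Storage is an interactable storage actor where the player buys items with coins through an options menu.
; Selecting Metal or Misc swaps the menu to that category's items.
; Any other option is mapped through OptionNameToID to an ItemData row for its price.
; If the player has enough coins and inventory space, the item is granted and coins deducted via controller messages.
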(event Custom|GivePlayerItem
  (params (Target :type Object%20Object%20Reference) (ItemID :type String))
  (Class|IController|GiveItem(Message) Target ItemID))

(event EventBeginPlay
  (|CallParentFunction) ; This node is disabled and will not be called.\nDrag off pins to build functionality.
)

(event Collision|EventActorBeginOverlap
  (params (OtherActor :type Actor%20Object%20Reference)))

(event EventTick
  (params (DeltaSeconds :type Float%20%28single-precision%29)))

(event EventOptionSelected
  (params (Option :type String))
  (bind _menu (Variables|Default|GetMenu))
  (switch string Option
    (:Default
      (bind _controller (Class|IGamemode|GetPlayerController(Message) (Game|GetGameMode)))
      (bind _total (Class|IController|GetPlayerCoins(Message) _controller))
      (bind _value (CallFunction|GetItemValue (Utilities|Text|ToText(String) Option)))
      (if (>= _total _value)
        (bind _isfull (Class|IController|GetInventory(Message) _controller))
        (if (not _isfull)
          (CallFunction|GivePlayerItem _controller (.Value (Utilities|Map|Find (Variables|Default|GetOptionNameToID) Option)))
          (Class|IController|ModifyCoins(Message) _controller (- 0 _value)))))
    (:Metal
      (Default|SetOptions _menu (Utilities|Array|MakeArray "Iron" "Gold" "Tin" "Copper")))
    (:Misc
      (Default|SetOptions _menu (Utilities|Array|MakeArray "Wood" "Coal" "Gems" "Flint")))))

(event EventOptionsMenuOpened
  (|CallParentFunction))

(fn ConstructionScript
  (|CallParentFunction))

(fn GetItemValue
  (params (ItemName :type Text))
  (bind _returnvalue (Utilities|GetDataTableRow (Variables|Default|GetItemData) (Utilities|String|StringToName (.Value (Utilities|Map|Find (Variables|Default|GetOptionNameToID) (Utilities|String|ToString(Text) ItemName)))))
    (:then
      (return (Utilities|Struct|BreaksItemData _returnvalue)))
    (:RowNotFound
      (return 0))))