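; BP_Daylight is a daylight actor that changes a directional light's colour and brightness with the in-game time of day.
; Each tick it reads the minutes from the game mode's date-and-time message, shifts them back six hours and wraps them to one day.
; The normalised time samples a colour curve: RGB times a tint sets the colour, alpha times a multiplier sets intensity.
; Construction applies indirect and volumetric scattering intensities.
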(event Custom|AdjustDayLight
  (bind _localtime (Variables|Default|GetLocalTime))
  (bind _colourcurve (Variables|Default|GetColourCurve))
  (bind _directionallight (Variables|Default|GetDirectionalLight))
  (bind _lighttint (Variables|LightSettings|GetLightTint))
  (bind _returnvalue (/ _localtime 1.44e+03))
  (bind _returnvalue_2 (Math|Curves|GetLinearColorValue _colourcurve _returnvalue))
  (bind _returnvalue_3 (* _returnvalue_2 _lighttint))
  (bind (_r _g _b) (Utilities|Struct|BreakLinearColor _returnvalue_3))
  (Rendering|Components|Light|SetLightColor _directionallight (Utilities|Struct|MakeLinearColor _r _g _b 1.0) true)
  (Rendering|Components|Light|SetIntensity _directionallight (* (Utilities|Struct|BreakLinearColor _returnvalue_2) (Variables|LightSettings|GetBrightnessMultiplier))))

(event EventBeginPlay)

(event EventTick
  (params (DeltaSeconds :type Float%20%28single-precision%29))
  (bind _timeinminutes (Class|IGamemode|GetDateandTime(Message) (Game|GetGameMode)))
  (bind _output_get (Variables|Default|SetLocalTime (- _timeinminutes 3.6e+02)))
  (if (< _output_get 0.0)
    (Variables|Default|SetLocalTime (+ (Variables|Default|GetLocalTime) 1.44e+03))
    (elif (> _output_get 1.44e+03)
      (Variables|Default|SetLocalTime (- (Variables|Default|GetLocalTime) 1.44e+03))))
  (CallFunction|AdjustDayLight))

(fn ConstructionScript
  (bind _directionallight (Variables|Default|GetDirectionalLight))
  (Class|LightComponent|SetIndirectLightingIntensity _directionallight (Variables|LightSettings|GetIndirectLightIntensity))
  (Class|LightComponent|SetVolumetricScatteringIntensity _directionallight (Variables|LightSettings|GetVolumetricScatteringIntensity)))