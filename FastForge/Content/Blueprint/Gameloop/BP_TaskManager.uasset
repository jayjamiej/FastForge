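; Task manager for the blacksmith game that guides the player step by step through crafting each customer's order.
; On a new order it recursively expands RecipeData into a task list, then reverses it into crafting order.
; Inventory additions advance, skip or reset the current task, updating the HUD message and highlighted station, ending at the Counter.
; Tanning or Storage tasks with zero coins start a delayed game-over timer.
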(event Custom|NewOrder
  (params (Customer :type BP%20Customer%20Character%20Object%20Reference))
  (bind _output_get (Variables|Default|SetCurrentCustomer Customer))
  (EventDispatchers|BindEventtoOrderComplete _output_get (delegate Custom|BindOrderComplete))
  (Utilities|FlowControl|Delay 0.5)
  (Variables|Default|SetCurrent 0)
  (bind _output_get_2 (Variables|Default|SetTarget (Variables|/Game/Blueprint/AI/BP_Customer_Character.BP_Customer_Character_C|GetOrder (Variables|Default|GetCurrentCustomer))))
  (bind _returnvalue (Utilities|GetDataTableRow (Variables|Default|GetItems) (Utilities|String|StringToName (Variables|/Game/Blueprint/AI/BP_Customer_Character.BP_Customer_Character_C|GetOrder (Variables|Default|GetCurrentCustomer))))
    (:then
      (Variables|Default|SetTargetName (.ItemName (Utilities|Struct|BreaksItemData _returnvalue))))
    (:RowNotFound
      _))
  (Utilities|Array|Clear (Variables|Default|GetTasks))
  (CallFunction|GetMachineOrder _output_get_2)
  (bind _out (CallFunction|ReverseArray (Variables|Default|GetTasks)))
  (bind _output_get_3 (Variables|Default|SetTasks _out))
  (CallFunction|DisplayTask (.Machine (Utilities|Struct|BreaksTask (Utilities|Array|Get(acopy) _output_get_3))) (.Output (Utilities|Struct|BreaksTask (Utilities|Array|Get(acopy) _output_get_3)))))

(event Custom|CharacterItemAdded
  (params (ItemID :type String) (Inventory :type Array%20of%20Strings))
  (if (Utilities|Enum|Equal(Enum) ItemID (.Output (Utilities|Struct|BreaksTask (Utilities|Array|Get(acopy) (Variables|Default|GetTasks) (Variables|Default|GetCurrent)))))
    (bind (_machine _taskindex _output _found) (CallFunction|FindNextTask Inventory :!label _label))
    (if _found
      (CallFunction|DisplayTask _machine _output)
      (Variables|Default|SetCurrent _taskindex)
      (elif (>= (Variables|Default|GetCurrent) (Utilities|Array|LastIndex (Variables|Default|GetTasks)))
        (CallFunction|HideAllPlayerCircles)
        (Default|ShowPlayerLocation (Variables|Default|GetCounter) true)
        (bind _returnvalue (Utilities|GetDataTableRow (Variables|Default|GetItems) (Utilities|String|StringToName (Variables|Default|GetTarget)))
          (:then
            (bind _controller (Class|IGamemode|GetPlayerController(Message) (Game|GetGameMode)))
            (Class|IController|NewTask(Message) _controller (Utilities|String|Append "Put the " (Utilities|String|ToString(Name) (.ItemName (Utilities|Struct|BreaksItemData _returnvalue))) " on the Counter") (Utilities|String|ToString(Name) (Variables|Default|GetTargetName)))))
        (else
          (bind _output_get (Variables|Default|SetCurrent (+ (Variables|Default|GetCurrent) 1)))
          (CallFunction|DisplayTask (.machine (Utilities|Array|Get(acopy) (Variables|Default|GetTasks) _output_get)) (.output (Utilities|Array|Get(acopy) (Variables|Default|GetTasks) _output_get))))))
    (else
      (bind _true (CallFunction|IsNewItemAnyTask ItemID Inventory))
      (if _true
        (goto _label)
        (else
          (bind _true_2 (CallFunction|CanStillCompleteTask Inventory))
          (if (not _true_2)
            (bind _output_get_2 (Variables|Default|SetCurrent 0))
            (CallFunction|DisplayTask (.machine (Utilities|Array|Get(acopy) (Variables|Default|GetTasks) _output_get_2)) (.output (Utilities|Array|Get(acopy) (Variables|Default|GetTasks) _output_get_2)))))))))

(event Custom|DisplayTask
  (params (Selection :type eMachineType%20Enum :default "NewEnumerator0") (Output :type String))
  (bind _gameovertimer (Variables|Default|GetGameOverTimer))
  (if (Utilities|Time|IsValidTimerHandle _gameovertimer)
    (Utilities|Time|ClearandInvalidateTimerbyHandle _gameovertimer))
  (if (or (Utilities|Enum|Equal(Enum) Selection "NewEnumerator3") (Utilities|Enum|Equal(Enum) Selection "NewEnumerator5"))
    (CallFunction|CoinCheck))
  (bind _controller (Class|IGamemode|GetPlayerController(Message) (Game|GetGameMode)))
  (bind _returnvalue (Utilities|GetDataTableRow (Variables|Default|GetItems) (Utilities|String|StringToName Output))
    (:then
      (Class|IController|NewTask(Message) _controller (Utilities|String|Append (Utilities|Select :Index Selection :NewEnumerator0 "Forge a " :NewEnumerator1 "Assemble the " :NewEnumerator2 "Finish the " :NewEnumerator3 "Gather " :NewEnumerator5 "Fetch the ") (Utilities|String|ToString(Name) (.ItemName (Utilities|Struct|BreaksItemData _returnvalue))) (Utilities|Select :Index Selection :NewEnumerator0 " in the Furnace" :NewEnumerator1 " at the Workbench" :NewEnumerator2 " at the Grindstone" :NewEnumerator3 " from the Tanning Rack" :NewEnumerator5 " from Storage")) (Utilities|String|ToString(Name) (Variables|Default|GetTargetName))))
    (:RowNotFound
      _))
  (CallFunction|HideAllPlayerCircles)
  (switch Utilities|FlowControl|Switch|SwitchoneMachineType Selection
    (:NewEnumerator0
      (Default|ShowPlayerLocation (Variables|Default|GetFurnace) true))
    (:NewEnumerator1
      (Default|ShowPlayerLocation (Variables|Default|GetWorkbench) true))
    (:NewEnumerator2
      (Default|ShowPlayerLocation (Variables|Default|GetGrindstone) true))
    (:NewEnumerator3
      (Default|ShowPlayerLocation (Variables|Default|GetTanningRack) true))
    (:NewEnumerator5
      (Default|ShowPlayerLocation (Variables|Default|GetStorage) true))))

(event Custom|BindOrderComplete
  (bind _controller (Class|IGamemode|GetPlayerController(Message) (Game|GetGameMode)))
  (Class|IController|HideTasks(Message) _controller))

(event Custom|CoinCheck
  (Utilities|FlowControl|Delay 0.2)
  (if (== (Variables|/Game/Blueprint/Player/BP_Blacksmith_Con.BP_Blacksmith_Con_C|GetCoins (Variables|Default|GetPlayerController)) 0)
    (bind _returnvalue (Utilities|Time|SetTimerbyEvent (delegate Custom|NoMoneyGameOver) 1e+01))
    (Variables|Default|SetGameOverTimer _returnvalue)))

(event Custom|NoMoneyGameOver
  (Class|IGamemode|GameOver(Message) (Game|GetGameMode)))

(event EventBeginPlay
  (EventDispatchers|BindEventtoOnNewCustomer (Variables|Default|GetQueue) (delegate Custom|NewOrder))
  (bind _controller (Class|IGamemode|GetPlayerController(Message) (Game|GetGameMode)))
  (bind _asbp_blacksmith_con (Utilities|Casting|CastToBP_Blacksmith_Con _controller))
  (bind _output_get (Variables|Default|SetPlayerController _asbp_blacksmith_con))
  (EventDispatchers|BindEventtoOnItemAdded _output_get (delegate Custom|CharacterItemAdded)))

(fn ConstructionScript)

(fn GetMachineOrder
  (params (ID_ToFind :type String))
  (bind _outrownames (DataTable|GetDataTableRowNames (Variables|Default|GetRecipeData)))
  (for _array_element _outrownames
    (bind _returnvalue (Utilities|GetDataTableRow (Variables|Default|GetRecipeData) _array_element)
      (:then
        (if (.ReturnValue (Utilities|Map|Find (.OptionsAndTime (Utilities|Struct|BreaksRecipes _returnvalue)) ID_ToFind))
          (Utilities|Array|Add (Variables|Default|GetTasks) (Utilities|Struct|MakesTask (.InputItem_1 (Utilities|Struct|BreaksRecipes _returnvalue)) (.InputItem_2 (Utilities|Struct|BreaksRecipes _returnvalue)) (.Machine (Utilities|Struct|BreaksRecipes _returnvalue)) ID_ToFind))
          (CallFunction|GetMachineOrder (.InputItem_2 (Utilities|Struct|BreaksRecipes _returnvalue)))
          (CallFunction|GetMachineOrder (.InputItem_1 (Utilities|Struct|BreaksRecipes _returnvalue)))
          (return true)))))
  (return false))

(fn ReverseArray
  (params (Array :type Array%20of%20S%20Task%20Structures))
  (bind _l_tasks (LocalVariables|GetL_Tasks))
  (bind _arrayelement (Utilities|Array|ReverseforEachLoop Array)
    (:LoopBody
      (Utilities|Array|Add _l_tasks _arrayelement))
    (:Completed
      (return _l_tasks))))

(fn HideAllPlayerCircles
  (Default|ShowPlayerLocation (Variables|Default|GetFurnace) false)
  (Default|ShowPlayerLocation (Variables|Default|GetWorkbench) false)
  (Default|ShowPlayerLocation (Variables|Default|GetStorage) false)
  (Default|ShowPlayerLocation (Variables|Default|GetTanningRack) false)
  (Default|ShowPlayerLocation (Variables|Default|GetGrindstone) false)
  (Default|ShowPlayerLocation (Variables|Default|GetCounter) false))

(fn FindNextTask
  (params (Inventory :type Array%20of%20Strings))
  (for (_array_element _array_index) (Variables|Default|GetTasks)
    (if (or (Utilities|Array|Identical (Utilities|Array|MakeArray (.Input1 (Utilities|Struct|BreaksTask _array_element)) (.Input2 (Utilities|Struct|BreaksTask _array_element))) Inventory) (Utilities|Array|Identical (Utilities|Array|MakeArray (.Input2 (Utilities|Struct|BreaksTask _array_element)) (.Input1 (Utilities|Struct|BreaksTask _array_element))) Inventory))
      (return (.Machine (Utilities|Struct|BreaksTask _array_element)) _array_index (.Output (Utilities|Struct|BreaksTask _array_element)) true)))
  (return "NewEnumerator0" 0 "" false))

(fn IsNewItemAnyTask
  (params (NewItem :type String) (Inv :type Array%20of%20Strings))
  (LocalVariables|SetInventory Inv)
  (for (_array_element _array_index) (Variables|Default|GetTasks)
    (if (> _array_index (Variables|Default|GetCurrent))
      (if (!= (Utilities|Array|FindItem (LocalVariables|GetInventory) (.Input1 (Utilities|Struct|BreaksTask _array_element))) -1)
        (Development|PrintString "Found Input 1")
        (if (Utilities|Enum|NotEqual(Enum) (.Input2 (Utilities|Struct|BreaksTask _array_element)) "")
          (if (!= (Utilities|Array|FindItem (LocalVariables|GetInventory) (.Input2 (Utilities|Struct|BreaksTask _array_element))) -1)
            (return true _array_index))
          (else
            (return true _array_index))))))
  (return false -1))

(fn CanStillCompleteTask
  (params (Inv :type Array%20of%20Strings))
  (bind _current (Variables|Default|GetCurrent))
  (bind _tasks (Variables|Default|GetTasks))
  (bind _output (Utilities|Array|Get(acopy) _tasks _current))
  (bind (_input1 _input2) (Utilities|Struct|BreaksTask _output))
  (bind _returnvalue (Utilities|Array|FindItem Inv _input1))
  (if (!= _returnvalue -1)
    (if (Utilities|Enum|NotEqual(Enum) _input2 "")
      (return (Utilities|Enum|Equal(Enum) _input2 (Utilities|Array|Get(acopy) Inv (Utilities|Select :Index _returnvalue :Option%200 1 :Option%201 0))))
      (else
        (return true)))
    (else
      (return false))))