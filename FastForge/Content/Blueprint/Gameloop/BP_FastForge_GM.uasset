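; Game mode for FastForge that runs the shop's day cycle, tracking the day count and an in-game clock advanced by a one-second looping timer.
; NextDay resets time to 09:00 and opens the BP_Queue shop; EndDay, from 17:00, clears the queue and shows the end-of-day widget.
; Both switch every machine's menu type and re-arm each other's DoOnce gate.
; It also caches the DayLight light and player controller, and handles game over.
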(event Custom|IncrementTime
  (bind _output_get (Variables|Default|SetTime (+ (Variables|Default|GetTime) (Variables|Default|GetMinutesPerRealSecond))))
  (if (>= (Math|Conversions|ToFloat(Integer) (.hours (Class|KismetMathLibrary|FromMinutes _output_get))) 17.0)
    (CallFunction|EndDay)
    (elif (Variables|Default|GetEndOfDay)
      (if (== (.hours (Class|KismetMathLibrary|FromMinutes _output_get)) 9)
        (CallFunction|NextDay)))))

(event Custom|EndDay
  (Utilities|FlowControl|DoOnce false
    (:Completed
      (bind _outactors (Actor|GetAllActorsOfClass "/Game/Blueprint/AI/BP_Queue.BP_Queue_C"))
      (Default|ClearQueue (Utilities|Array|Get(acopy) _outactors))
      (bind _returnvalue (UserInterface|CreateWidget "/Game/Blueprint/UI/UI_EndOfDay.UI_EndOfDay_C" 0 self))
      (Variables|Default|SetNextDayHUD _returnvalue)
      (UserInterface|Viewport|AddtoViewport _returnvalue 0)
      (for _array_element (Variables|Default|GetMachines)
        (Default|SwitchMenuType _array_element "NewEnumerator1"))
      (Variables|Default|SetEndOfDay true)
      (CallFunction|ResetNextDay))))

(event Custom|NextDay
  (bind _nextdayhud (Variables|Default|GetNextDayHUD))
  (Utilities|FlowControl|DoOnce false
    (:Completed
      (Utilities|IsValid _nextdayhud
        (:Is%20Valid
          (Widget|RemovefromParent _nextdayhud))
        (:Is%20Not%20Valid
          _))
      (Math|Integer|IncrementInt (Variables|Default|GetDay)
        (:%20%20
          (Variables|Default|SetTime 5.4e+02)
          (for _array_element (Variables|Default|GetMachines)
            (Default|SwitchMenuType _array_element "NewEnumerator0"))
          (CallFunction|ResetEndOFDay)
          (bind _outactors (Actor|GetAllActorsOfClass "/Game/Blueprint/AI/BP_Queue.BP_Queue_C"))
          (Default|OpenShop (Utilities|Array|Get(acopy) _outactors)))))))

(event Custom|ResetEndOfDay
  (Utilities|FlowControl|DoOnce false) ; enters at Reset
)

(event Custom|ResetNextDay
  (bind _nextdayhud (Variables|Default|GetNextDayHUD))
  (Utilities|FlowControl|DoOnce false) ; enters at Reset
)

(event EventBeginPlay
  (bind _outactors (Actor|GetAllActorsOfClass "/Game/Blueprint/Machines/BP_Machine.BP_Machine_C"))
  (Variables|Default|SetMachines _outactors)
  (Utilities|FlowControl|Delay 0.5)
  (CallFunction|NextDay)
  (Utilities|Time|SetTimerbyEvent (delegate Custom|IncrementTime) 1.0 true)
  (bind _outactors_2 (Actor|GetAllActorsOfClass "/Script/Engine.DirectionalLight"))
  (for _array_element _outactors_2
    (if (Utilities|Enum|Equal(Enum) (Utilities|GetDisplayName _array_element) "DayLight")
      (Variables|Default|SetDayLight _array_element))))

(event EventGameOver
  (Game|OpenLevel(byName) "GameOver"))

(event EventPostLogin
  (params (NewPlayer :type Player%20Controller%20Object%20Reference))
  (Variables|Default|SetController NewPlayer))

(fn ConstructionScript)

(fn GetDateandTime
  (return (Variables|Default|GetTime) (Variables|Default|GetDay)))

(fn GetPlayerController
  (return (Variables|Default|GetController)))