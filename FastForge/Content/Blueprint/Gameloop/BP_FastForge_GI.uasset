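; Game instance for FastForge that holds player settings: controller scheme, difficulty multiplier and a flag for showing text instead of images.
; Each setting has a setter event that stores the value and a getter function that returns it.
; It contains no other logic, acting as a simple settings store shared across the game.
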(event EventSetControllerScheme
  (params (Scheme :type eControllerScheme%20Enum :default "NewEnumerator0"))
  (Variables|Default|SeteControllerScheme Scheme))

(event EventSetDifficulty
  (params (Multiplier :type Float%20%28single-precision%29))
  (Variables|Default|SetDifficultyMultiplier Multiplier))

(event EventSetUseText
  (params (True :type Boolean))
  (Variables|Default|SetUseTextNotImage True))

(fn GetControllerScheme
  (return (Variables|Default|GeteControllerScheme)))

(fn GetDifficulty
  (return (Variables|Default|GetDifficultyMultiplier)))

(fn GetUseText
  (return (Variables|Default|GetUseTextNotImage)))