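; Crafting machine that turns items from the player's inventory into a chosen result after a timed cook.
; BeginPlay filters the Recipes table by MachineType; opening the menu matches two inventory slots to a recipe and lists its outputs.
; Selection consumes inputs and shows a progress bar, optionally snapping and locking the player at an arrow.
; ResetOptions grants the finished item if the player is in range, using player controller messages.
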(event Custom|LockPlayer
  (params (Locked :type Boolean))
  (bind _arrow (Variables|Default|GetArrow))
  (bind _returnvalue (Transformation|GetWorldTransform _arrow))
  (if Locked
    (bind _controller (Class|IGamemode|GetPlayerController(Message) (Game|GetGameMode)))
    (Transformation|SetActorTransform (Pawn|GetControlledPawn _controller) (Math|Transform|MakeTransform (Math|Vector|MakeVector (.x (.location _returnvalue)) (.y (.location _returnvalue)) (.z (Transformation|GetActorLocation (Pawn|GetControlledPawn _controller)))) (.rotation _returnvalue) "1,1,1")))
  (Class|IController|LockPlayerMovement(Message) _controller Locked))

(event EventBeginPlay
  (|CallParentFunction)
  (bind _outrownames (DataTable|GetDataTableRowNames (Variables|Recipe|GetRecipes)))
  (for _array_element _outrownames
    (bind _returnvalue (Utilities|GetDataTableRow (Variables|Recipe|GetRecipes) _array_element)
      (:then
        (if (Utilities|Enum|Equal(Enum) (Utilities|Struct|BreaksRecipes _returnvalue) (Variables|Default|GetMachineType))
          (Utilities|Array|Add (Variables|Recipe|GetMachineRecipes) _returnvalue)))))
  (Development|PrintString (Utilities|String|Append (Utilities|GetObjectName self) " = " (Utilities|String|ToString(Integer) (Utilities|Array|Length (Variables|Recipe|GetMachineRecipes))) "recipes")))

(event Collision|EventActorBeginOverlap
  (params (OtherActor :type Actor%20Object%20Reference)))

(event EventTick
  (params (DeltaSeconds :type Float%20%28single-precision%29)))

(event EventOptionsMenuOpened
  (|CallParentFunction)
  (bind _controller (Class|IGamemode|GetPlayerController(Message) (Game|GetGameMode)))
  (bind _items (Class|IController|GetInventory(Message) _controller))
  (bind (_index _returninputs) (CallFunction|FindRecipeIndex _items))
  (Variables|Default|SetCanMenuOpen (!= _index -1))
  (Variables|Recipe|SetInputs _returninputs)
  (Variables|Recipe|SetRecipeIndex _index)
  (Development|PrintString (Utilities|String|Append (.InputItem_1 (Utilities|Struct|BreaksRecipes (Utilities|Array|Get(acopy) (Variables|Recipe|GetMachineRecipes) _index))) (Utilities|String|ToString(Integer) (Utilities|Map|Length (.OptionsAndTime (Utilities|Struct|BreaksRecipes (Utilities|Array|Get(acopy) (Variables|Recipe|GetMachineRecipes) _index)))))))
  (bind _keys (Utilities|Map|Keys (.OptionsAndTime (Utilities|Struct|BreaksRecipes (Utilities|Array|Get(acopy) (Variables|Recipe|GetMachineRecipes) _index)))))
  (bind _names (CallFunction|RecipetoNameArray _keys))
  (Default|SetDefaultOptions (Variables|Default|GetMenu) _names))

(event EventOptionSelected
  (params (Option :type String))
  (if (not (Variables|Cook|GetIsCooking))
    (if (Variables|Default|GetCanCook)
      (bind _controller (Class|IGamemode|GetPlayerController(Message) (Game|GetGameMode)))
      (for (_array_element _array_index) (Variables|Recipe|GetInputs)
        (if (Utilities|Enum|NotEqual(Enum) _array_element "")
          (bind _success (Class|IController|RemoveItem(Message) _controller _array_element))
          (if _success
            (if (and (Math|Boolean|Equal(Boolean) (Variables|Recipe|GetRecipeComplete) false) (== _array_index 1))
              (Variables|Recipe|SetRecipeComplete false)
              (else
                (Variables|Recipe|SetRecipeComplete true)))
            (else
              (Variables|Recipe|SetRecipeComplete false)))))
      (if (Variables|Recipe|GetRecipeComplete)
        (bind _output_get (Variables|Default|SetResult (.Value (Utilities|Map|Find (Variables|Default|GetOptionNameToID) Option))))
        (bind _returnvalue (UserInterface|CreateWidget "/Game/Blueprint/UI_ProgressBar.UI_ProgressBar_C" 0 (.Value (Utilities|Map|Find (Utilities|Struct|BreaksRecipes (Utilities|Array|Get(acopy) (Variables|Recipe|GetMachineRecipes) (Variables|Recipe|GetRecipeIndex))) _output_get))))
        (Variables|Default|SetProgress _returnvalue)
        (UserInterface|SetWidget (Variables|Default|GetWidget) _returnvalue)
        (Variables|Cook|SetIsCooking true)
        (Variables|Cook|SetCookFinishTime (+ (Utilities|Time|GetTimeSeconds) (.Value (Utilities|Map|Find (Utilities|Struct|BreaksRecipes (Utilities|Array|Get(acopy) (Variables|Recipe|GetMachineRecipes) (Variables|Recipe|GetRecipeIndex))) _output_get))))
        (Variables|Default|SetCanMenuOpen false)
        (if (Variables|Cook|GetLockPlayerDuringCook)
          (CallFunction|LockPlayer true))))))

(event EventResetOptions
  (if (Variables|Cook|GetIsCooking)
    (if (>= (Utilities|Time|GetTimeSeconds) (Variables|Cook|GetCookFinishTime))
      (bind _controller (Class|IGamemode|GetPlayerController(Message) (Game|GetGameMode)))
      (if (Collision|IsOverlappingActor (Variables|Default|GetPlayerRadius) (Pawn|GetControlledPawn _controller) :!class /Script/Engine.PrimitiveComponent)
        (bind _success (Class|IController|GiveItem(Message) _controller (Variables|Default|GetResult)))
        (if _success
          (UserInterface|SetWidget (Variables|Default|GetWidget) 0)
          (Variables|Cook|SetIsCooking false)
          (Variables|Default|SetCanMenuOpen true)
          (CallFunction|LockPlayer false))))
    (else
      (|CallParentFunction))))

(fn ConstructionScript
  (|CallParentFunction))

(fn FindRecipeIndex
  (params (Inventory :type Array%20of%20Strings))
  (bind _output (Utilities|Array|Get(acopy) Inventory 1))
  (bind _output_2 (Utilities|Array|Get(acopy) Inventory))
  (for (_array_element _array_index) (Variables|Recipe|GetMachineRecipes)
    (LocalVariables|SetCurrentIndex _array_index)
    (Development|PrintString (Utilities|String|Append (.InputItem_1 (Utilities|Struct|BreaksRecipes _array_element)) " + " (.InputItem_2 (Utilities|Struct|BreaksRecipes _array_element))))
    (LocalVariables|SetInput_Local (Utilities|Array|MakeArray (.InputItem_1 (Utilities|Struct|BreaksRecipes _array_element)) (.InputItem_2 (Utilities|Struct|BreaksRecipes _array_element))))
    (if (or (Utilities|Enum|Equal(Enum) (.InputItem_1 (Utilities|Struct|BreaksRecipes _array_element)) _output_2) (Utilities|Enum|Equal(Enum) (.InputItem_1 (Utilities|Struct|BreaksRecipes _array_element)) _output))
      (if (Utilities|Enum|Equal(Enum) (.InputItem_2 (Utilities|Struct|BreaksRecipes _array_element)) "")
        (return (LocalVariables|GetCurrentIndex) (LocalVariables|GetInput_Local))
        (elif (Utilities|Enum|Equal(Enum) (.InputItem_1 (Utilities|Struct|BreaksRecipes _array_element)) _output_2)
          (if (Utilities|Enum|Equal(Enum) _output (.InputItem_2 (Utilities|Struct|BreaksRecipes _array_element)))
            (return (LocalVariables|GetCurrentIndex) (LocalVariables|GetInput_Local)))
          (elif (Utilities|Enum|Equal(Enum) _output_2 (.InputItem_2 (Utilities|Struct|BreaksRecipes _array_element)))
            (return (LocalVariables|GetCurrentIndex) (LocalVariables|GetInput_Local)))))))
  (return -1 0))

(fn RecipetoNameArray
  (params (IDs :type Array%20of%20Strings))
  (bind _items (LocalVariables|GetItems))
  (for _index (range 0 3)
    (Development|PrintString (Utilities|Array|Get(acopy) IDs _index))
    (bind _returnvalue (Utilities|GetDataTableRow (Variables|Default|GetItemData) (Utilities|String|StringToName (Utilities|Array|Get(acopy) IDs _index)))
      (:then
        (Utilities|Array|Add _items (.ItemName (Utilities|Struct|BreaksItemData _returnvalue))))
      (:RowNotFound
        (Utilities|Array|Add _items ""))))
  (return (LocalVariables|GetItems)))