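; FastForge game mode that keeps a running game clock and a reference to the player controller.
; A looping one-second timer increments Time, which GetDateAndTime returns as minutes alongside Day, a value this graph never changes.
; PostLogin stores the joining controller for GetPlayerController to return, so each new login replaces the previous one.
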(event Custom|IncrementTime
  (Variables|Default|SetTime (+ (Variables|Default|GetTime) 1.0)))

(event EventBeginPlay
  (Utilities|Time|SetTimerbyEvent (delegate Custom|IncrementTime) 1.0 true))

(event EventTick
  (params (DeltaSeconds :type Float%20%28single-precision%29)))

(event EventPostLogin
  (params (NewPlayer :type Player%20Controller%20Object%20Reference))
  (Variables|Default|SetController NewPlayer))

(fn ConstructionScript)

(fn GetDateandTime
  (return (Variables|Default|GetTime) (Variables|Default|GetDay)))

(fn GetPlayerController
  (return (Variables|Default|GetController)))