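; Player blacksmith character that moves on world X/Y axes and shows the items it carries in its hands.
; On BeginPlay it takes walk speed from the controller, scales spring arm camera lag to match, and binds to the controller's item added and removed events.
; Inventory changes look up the first two items in ItemData to update two socket-attached meshes.
; It also exposes a coin rain particle trigger.
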(event Custom|InventoryChanged
  (params (ItemID :type String) (Inventory :type Array%20of%20Strings))
  (bind _item1 (Variables|Default|GetItem1))
  (bind _item2 (Variables|Default|GetItem2))
  ;[1 1 1] Displays items in the player's inventory on the player's hands
  (bind _returnvalue (Utilities|GetDataTableRow (Variables|Default|GetItemData) (Utilities|String|StringToName (Utilities|Array|Get(acopy) Inventory)))
    (:then
      (Components|StaticMesh|SetStaticMesh _item1 (.ItemMesh (Utilities|Struct|BreaksItemData _returnvalue)))
      (Utilities|IsValid (.ItemMeshMaterial (Utilities|Struct|BreaksItemData _returnvalue))
        (:Is%20Valid
          (Rendering|Material|SetMaterial (Variables|Default|GetItem1) 0 (.ItemMeshMaterial (Utilities|Struct|BreaksItemData _returnvalue))))
        (:Is%20Not%20Valid
          _))
      (bind _returnvalue_2 (Utilities|GetDataTableRow (Variables|Default|GetItemData) (Utilities|String|StringToName (Utilities|Array|Get(acopy) Inventory 1)))
        (:then
          (Components|StaticMesh|SetStaticMesh _item2 (.ItemMesh (Utilities|Struct|BreaksItemData _returnvalue_2)))
          (Utilities|IsValid (.ItemMeshMaterial (Utilities|Struct|BreaksItemData _returnvalue_2))
            (:Is%20Valid
              (Rendering|Material|SetMaterial (Variables|Default|GetItem2) 0 (.ItemMeshMaterial (Utilities|Struct|BreaksItemData _returnvalue_2))))))
        (:RowNotFound
          (Components|StaticMesh|SetStaticMesh _item2 0))))
    (:RowNotFound
      (Components|StaticMesh|SetStaticMesh _item1 0)
      (Components|StaticMesh|SetStaticMesh (Variables|Default|GetItem2) 0))))

(event Custom|ItemRemoved
  (params (ItemRemoved :type String) (Inventory :type Array%20of%20Strings) (ForRecipe :type Boolean))
  ;[1 1 1] Inits character to controller
  (CallFunction|InventoryChanged ItemRemoved Inventory))

(event EventBeginPlay
  ;[1 1 1] Inits character to controller
  (CallFunction|SetUpCharacterStats)
  (bind _asbp_blacksmith_con (Utilities|Casting|CastToBP_Blacksmith_Con (Pawn|GetController)))
  (EventDispatchers|BindEventtoOnItemAdded _asbp_blacksmith_con (EventDispatchers|CreateEvent :!event Custom|InventoryChanged))
  (EventDispatchers|BindEventtoOnItemRemoved _asbp_blacksmith_con (delegate Custom|ItemRemoved)))

(event EventShowCoins
  (Components|Activation|Activate (Variables|Default|GetPS_CoinRain) false))

(event EventMoveRight
  (params (Axis :type Float%20%28single-precision%29))
  (Class|PawnMovementComponent|AddInputVector (Variables|Character|GetCharacterMovement) (Math|Vector|MakeVector 0.0 Axis 0.0) false))

(event EventMoveForward
  (params (Axis :type Float%20%28single-precision%29))
  (Class|PawnMovementComponent|AddInputVector (Variables|Character|GetCharacterMovement) (Math|Vector|MakeVector Axis 0.0 0.0) false))

(fn ConstructionScript
  (Transformation|AttachComponentToComponent (Variables|Default|GetItem1) (Variables|Character|GetMesh) "Inv_1" "SnapToTarget" "SnapToTarget" "KeepWorld" true)
  (Transformation|AttachComponentToComponent (Variables|Default|GetItem2) (Variables|Character|GetMesh) "Inv_2" "SnapToTarget" "SnapToTarget" "KeepWorld" true))

(fn SetUpCharacterStats
  (bind _speed (Class|IController|GetCharacterStats(Message) (Pawn|GetController)))
  (Variables|/Script/Engine.CharacterMovementComponent|SetMaxWalkSpeed (Variables|Character|GetCharacterMovement) _speed)
  (Variables|/Script/Engine.SpringArmComponent|SetCameraLagSpeed (Variables|Default|GetSpringArm) (* (/ _speed 5e+02) 2.0)))

(fn GetMeshComponent
  (return (Variables|Character|GetMesh)))