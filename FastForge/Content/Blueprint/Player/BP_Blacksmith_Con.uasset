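; Player controller for the blacksmith character, handling click-to-move input and holding inventory, coins and animation state.
; On BeginPlay it creates the custom cursor and HUD, then broadcasts the starting coin count.
; Mouse clicks trace under the cursor and use SimpleMoveToLocation unless movement is locked.
; Functions manage a capacity-limited item ID inventory and coin changes, which notify listeners and show a pawn message on gains.
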(event Custom|GiveItem_1_1
  (params (ItemID :type String)))

(event EventBeginPlay
  (bind _returnvalue (UserInterface|CreateWidget "/Game/Blueprint/UI/UI_Cursor.UI_Cursor_C" self))
  (Class|PlayerController|SetMouseCursorWidget "Default" _returnvalue)
  (Variables|Default|SetbShowMouseCursor true)
  (bind _returnvalue_2 (UserInterface|CreateWidget "/Game/Blueprint/UI/UI_HUD.UI_HUD_C" 0 self))
  (UserInterface|Viewport|AddtoViewport _returnvalue_2 0)
  (Default|CallOnCoinsChanged (Variables|Inventory|GetCoins)))

(event EventTick
  (params (DeltaSeconds :type Float%20%28single-precision%29)))

(event EventSetAnimationState
  (params (State :type eAnimState%20Enum :default "NewEnumerator0"))
  (Variables|Default|SetState State))

(event EventLockPlayerMovement
  (params (Locked :type Boolean))
  (Variables|Default|SetCanMove (not Locked)))

(event Input|ActionEvents|InputActionMouseSelect
  (params (Key :type Key%20Structure :default "None"))
  (bind (_hitresult _returnvalue) (Game|Player|GetHitResultUnderCursorbyChannel "TraceTypeQuery1" true))
  (:Pressed
    (if _returnvalue
      (CallFunction|TryCharacterMove (.Location (Collision|BreakHitResult _hitresult))))))

(fn ConstructionScript)

(fn GetAnimState
  (return (Variables|Default|GetState)))

(fn GetCharacterStats
  (return (Variables|Character|GetCharacterSpeed)))

(fn GetInventory
  (bind _inventory (Variables|Inventory|GetInventory))
  (return _inventory (== (Utilities|Array|Length _inventory) (Variables|Character|GetMaxInventory))))

(fn GetPlayerCoins
  (return (Variables|Inventory|GetCoins)))

(fn GiveItem
  (params (ItemID :type String))
  (if (< (Utilities|Array|Length (Variables|Inventory|GetInventory)) (Variables|Character|GetMaxInventory))
    (Utilities|Array|Add (Variables|Inventory|GetInventory) ItemID)
    (return true)
    (else
      (return false))))

(fn ModifyCoins
  (params (In :type Integer))
  (bind _output_get (Variables|Inventory|SetCoins (+ (Variables|Inventory|GetCoins) In)))
  (Default|CallOnCoinsChanged _output_get In)
  (if (> In 0)
    (Class|IPawn|ShowCoins(Message) (Pawn|GetControlledPawn)))
  (return _output_get))

(fn RemoveItem
  (params (ItemID :type String))
  (bind _inventory (Variables|Inventory|GetInventory))
  (for (_array_element _array_index) _inventory
    (if (Utilities|Enum|Equal(Enum) _array_element ItemID)
      (if (== (LocalVariables|GetIndex) -1)
        (LocalVariables|SetIndex _array_index))))
  (if (== (LocalVariables|GetIndex) -1)
    (return false)
    (else
      (Utilities|Array|RemoveIndex _inventory (LocalVariables|GetIndex))
      (return true))))

(fn TryCharacterMove
  (params (Location :type Vector :default "0, 0, 0"))
  (if (Variables|Default|GetCanMove)
    (AI|Navigation|SimpleMovetoLocation self Location))
  (return (Variables|Default|GetCanMove)))