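; BP_CustomerController is an AI controller for customer characters that moves them to a requested location.
; TryCharacterMove prints the target location, calls MoveToLocation and always returns true, leaving an older SimpleMoveToLocation call disconnected.
; The animation state, stats, inventory, coin and item functions are stubs that return fixed defaults, and the event graph holds no logic.
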(event EventBeginPlay)

(fn ConstructionScript)

(fn GetAnimState
  (return "NewEnumerator0"))

(fn GetCharacterStats
  (return 0.0))

(fn GetInventory
  (return 0 false))

(fn GetPlayerCoins
  (return 0))

(fn GiveItem
  (params (ItemID :type String))
  (return false))

(fn ModifyCoins
  (params (In :type Integer))
  (return 0))

(fn RemoveItem
  (params (ItemID :type String))
  (return false))

(fn TryCharacterMove
  (params (Location :type Vector :default "0, 0, 0"))
  (Development|PrintString (Utilities|String|ToString(Vector) Location))
  (AI|Navigation|MovetoLocation Location -1.0 true true false true 0)
  (return true))