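; BP_Shutter is a shutter actor that opens and closes on OpenShutter and CloseShutter events.
; A timeline named Open plays forward to close and in reverse to open, at a rate set from the PlayRate variable on BeginPlay.
; Its single vector track drives the relative yaw of three shutter meshes, one vector component per mesh.
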(event Custom|OpenShutter
  (bind _z_axis (Timeline|Open Reverse)
    (:Update
      (Transformation|SetRelativeRotation (Variables|Default|GetSM_ShutterTest) (Math|Rotator|MakeRotator 0.0 0.0 (.x _z_axis)) false false)
      (Transformation|SetRelativeRotation (Variables|Default|GetSM_ShutterTest1) (Math|Rotator|MakeRotator 0.0 0.0 (.y _z_axis)) false false)
      (Transformation|SetRelativeRotation (Variables|Default|GetSM_ShutterTest2) (Math|Rotator|MakeRotator 0.0 0.0 (.z _z_axis)) false false))))

(event Custom|CloseShutter
  (bind _z_axis (Timeline|Open Play)
    (:Update
      (Transformation|SetRelativeRotation (Variables|Default|GetSM_ShutterTest) (Math|Rotator|MakeRotator 0.0 0.0 (.x _z_axis)) false false)
      (Transformation|SetRelativeRotation (Variables|Default|GetSM_ShutterTest1) (Math|Rotator|MakeRotator 0.0 0.0 (.y _z_axis)) false false)
      (Transformation|SetRelativeRotation (Variables|Default|GetSM_ShutterTest2) (Math|Rotator|MakeRotator 0.0 0.0 (.z _z_axis)) false false))))

(event EventBeginPlay
  (Components|Timeline|SetPlayRate (Variables|Default|GetOpen) (Variables|Default|GetPlayRate)))

(fn ConstructionScript)