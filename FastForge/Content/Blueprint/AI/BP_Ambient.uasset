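; BP_Ambient is an ambient AI character that walks slowly forward with a randomized appearance for a short, fixed lifetime.
; On BeginPlay it picks a random Outfits data table row and applies a random material, hair and accessory from it to that row's base mesh.
; Hair and accessory meshes attach to the Head socket in construction.
; A timer destroys controller and character, and Tick prints time since spawn while falling.
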(event Custom|Dead
  (Actor|DestroyActor (Pawn|GetController))
  (Actor|DestroyActor))

(event EventBeginPlay
  (bind _look (CallFunction|GetRandomLook (Variables|Default|GetOutfits)))
  (CallFunction|SetLook _look)
  (Variables|Default|SetSpawnTime (Utilities|Time|GetGameTimeinSeconds))
  (Utilities|Time|SetTimerbyEvent (delegate Custom|Dead) 15.0))

(event Collision|EventActorBeginOverlap
  (params (OtherActor :type Actor%20Object%20Reference)))

(event EventTick
  (params (DeltaSeconds :type Float%20%28single-precision%29))
  (Pawn|Input|AddMovementInput (Transformation|GetActorForwardVector) 0.2 false)
  (if (AI|Components|NavMovement|IsFalling (Variables|Character|GetCharacterMovement))
    (Development|PrintString (Utilities|String|ToString(Float) (- (Utilities|Time|GetGameTimeinSeconds) (Variables|Default|GetSpawnTime))))))

(fn ConstructionScript
  (Transformation|AttachComponentToComponent (Variables|Default|GetAccessory) (Variables|Character|GetMesh) "Head" "SnapToTarget" "KeepWorld" "KeepRelative" true)
  (Transformation|AttachComponentToComponent (Variables|Default|GetHair) (Variables|Character|GetMesh) "Head" "SnapToTarget" "KeepWorld" "KeepRelative" true))

(fn GetRandomLook
  (params (NewParam1 :type Data%20Table%20Object%20Reference))
  (bind _outrownames (DataTable|GetDataTableRowNames NewParam1))
  (LocalVariables|SetRows _outrownames)
  (bind _returnvalue (Utilities|GetDataTableRow (Variables|Default|GetOutfits) (Utilities|Array|Get(acopy) (LocalVariables|GetRows) (Math|Random|RandomIntegerinRange 0 (Utilities|Array|LastIndex (LocalVariables|GetRows)))))
    (:then
      (return _returnvalue))))

(fn SetLook
  (params (Look :type S%20Customer%20Looks%20Structure))
  (bind _hair (Variables|Default|GetHair))
  (bind _accessory (Variables|Default|GetAccessory))
  (bind _output_get (LocalVariables|Setl_Look Look))
  (Class|SkinnedMeshComponent|SetSkeletalMesh (Variables|Character|GetMesh) (Utilities|Struct|BreaksCustomerLooks _output_get) true)
  (Rendering|Material|SetMaterial (Variables|Character|GetMesh) 0 (Utilities|Array|Get(acopy) (Utilities|Struct|BreaksCustomerLooks (LocalVariables|Getl_Look)) (Math|Random|RandomIntegerinRange 0 (Utilities|Array|LastIndex (Utilities|Struct|BreaksCustomerLooks (LocalVariables|Getl_Look))))))
  (Components|StaticMesh|SetStaticMesh _hair (Utilities|Array|Get(acopy) (.HairPieces (Utilities|Struct|BreaksCustomerLooks (LocalVariables|Getl_Look))) (Math|Random|RandomIntegerinRange 0 (Utilities|Array|LastIndex (.HairPieces (Utilities|Struct|BreaksCustomerLooks (LocalVariables|Getl_Look)))))))
  (Utilities|IsValid (Variables|/Script/Engine.StaticMeshComponent|GetStaticMesh _hair)
    (:Is%20Valid
      (Rendering|Material|SetMaterial (Variables|Default|GetHair) 0 (Utilities|Array|Get(acopy) (.HairMaterials (Utilities|Struct|BreaksCustomerLooks (LocalVariables|Getl_Look))) (Math|Random|RandomIntegerinRange 0 (Utilities|Array|LastIndex (.HairMaterials (Utilities|Struct|BreaksCustomerLooks (LocalVariables|Getl_Look))))))))
    (:Is%20Not%20Valid
      _))
  (Components|StaticMesh|SetStaticMesh _accessory (Utilities|Array|Get(acopy) (.Accessories (Utilities|Struct|BreaksCustomerLooks (LocalVariables|Getl_Look))) (Math|Random|RandomIntegerinRange 0 (Utilities|Array|LastIndex (.Accessories (Utilities|Struct|BreaksCustomerLooks (LocalVariables|Getl_Look)))))))
  (Utilities|IsValid (Variables|/Script/Engine.StaticMeshComponent|GetStaticMesh _accessory)
    (:Is%20Valid
      (Rendering|Material|SetMaterial _accessory 0 (Utilities|Array|Get(acopy) (.AccessoryMaterials (Utilities|Struct|BreaksCustomerLooks (LocalVariables|Getl_Look))) (Math|Random|RandomIntegerinRange 0 (Utilities|Array|LastIndex (.AccessoryMaterials (Utilities|Struct|BreaksCustomerLooks (LocalVariables|Getl_Look))))))))))