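; Customer queue actor for a shop that spawns AI customers and lines them up at a counter.
; Construction lays out arrow components as queue slots; opening the shop raises shutters and staggers the first four spawns on random timers.
; The front customer shows its order on reaching the counter; when one is destroyed, the line advances and a replacement spawns at the back.
; Closing sends customers to the exit, then destroys them.
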(event OnComponentBeginOverlap(CounterRadius)
  (params (OverlappedComponent :type Primitive%20Component%20Object%20Reference) (OtherActor :type Actor%20Object%20Reference) (OtherComp :type Primitive%20Component%20Object%20Reference) (OtherBodyIndex :type Integer) (bFromSweep :type Boolean) (SweepResult :type Hit%20Result%20Structure%20%28by%20ref%29))
  (bind _customers (Variables|Default|GetCustomers))
  (bind _output (Utilities|Array|Get(acopy) _customers))
  (if (== OtherActor _output)
    (Utilities|FlowControl|Delay 0.2)
    (Transformation|SetActorRotation OtherActor (Transformation|GetWorldRotation (Variables|Default|GetArrow)))
    (Default|ShowOrder _output (Variables|Default|GetCounter))
    (Default|CallOnNewCustomer _output)))

(event Custom|OrderFulfilled
  (params (DestroyedActor :type Actor%20Object%20Reference))
  (bind _customers (Variables|Default|GetCustomers))
  (bind _queuepositions (Variables|Default|GetQueuePositions))
  (bind _asbp_customer_character (Utilities|Casting|CastToBP_Customer_Character DestroyedActor))
  (Utilities|Array|RemoveIndex _customers (Utilities|Array|FindItem _customers _asbp_customer_character))
  (for (_array_element _array_index) (Variables|Default|GetCustomers)
    (Utilities|IsValid _array_element
      (:Is%20Valid
        (Class|IController|TryCharacterMove(Message) (Pawn|GetController _array_element) (.location (Transformation|GetWorldTransform (Utilities|Array|Get(acopy) (Variables|Default|GetQueuePositions) _array_index)))))))
  (if (Variables|Default|GetShopOpen)
    (Utilities|FlowControl|Delay (Math|Random|RandomFloatinRange 2.0 1e+01))
    (bind _returnvalue (Game|SpawnActorfromClass "/Game/Blueprint/AI/BP_Customer_Character.BP_Customer_Character_C" (Transformation|GetWorldTransform (Utilities|Array|Get(acopy) _queuepositions (Utilities|Array|LastIndex _queuepositions))) "AdjustIfPossibleButAlwaysSpawn" 0 self 0))
    (Utilities|Array|Add (Variables|Default|GetCustomers) _returnvalue)
    (Game|BindEventtoOnDestroyed _returnvalue (EventDispatchers|CreateEvent :!event Custom|OrderFulfilled))))

(event Custom|SlowSpawn
  (bind _initspawncount (Variables|Default|GetInitSpawnCount))
  (Math|Integer|IncrementInt _initspawncount
    (:%20%20
      (bind _returnvalue (Game|SpawnActorfromClass "/Game/Blueprint/AI/BP_Customer_Character.BP_Customer_Character_C" (Math|Transform|MakeTransform (CallFunction|GetSpawnLocation) "0, 0, 0" "1,1,1") "Undefined" 0 self 0))
      (Utilities|Array|Add (Variables|Default|GetCustomers) _returnvalue)
      (Game|BindEventtoOnDestroyed _returnvalue (EventDispatchers|CreateEvent :!event Custom|OrderFulfilled))
      (Utilities|IsValid (Pawn|GetController _returnvalue)
        (:Is%20Valid
          (Class|IController|TryCharacterMove(Message) (Pawn|GetController _returnvalue) (Transformation|GetWorldLocation (Utilities|Array|Get(acopy) (Variables|Default|GetQueuePositions) (- _initspawncount 1))))
          (if (!= (Variables|Default|GetInitSpawnCount) 4)
            (Utilities|Time|SetTimerbyEvent (EventDispatchers|CreateEvent :!event Custom|SlowSpawn) (Math|Random|RandomFloatinRange 1.0 1e+01))))))))

(event Custom|ClearQueue
  (bind _customers (Variables|Default|GetCustomers))
  (Variables|Default|SetShopOpen false)
  (for _array_element (Variables|Default|GetCustomers)
    (Utilities|IsValid _array_element
      (:Is%20Valid
        (Class|IController|TryCharacterMove(Message) (Pawn|GetController _array_element) (Variables|Default|GetExitLocation))
        (EventDispatchers|UnbindallEventsfromOnDestroyed _array_element))))
  (for _array_element_2 (Variables|Default|GetShutters)
    (Default|CloseShutter _array_element_2))
  (Utilities|FlowControl|Delay 2.0)
  (for _array_element_3 _customers
    (Actor|DestroyActor _array_element_3))
  (Utilities|Array|Clear _customers)
  (Variables|Default|SetInitSpawnCount 0))

(event Custom|OpenShop
  (Variables|Default|SetShopOpen true)
  (CallFunction|SlowSpawn)
  (for _array_element (Variables|Default|GetShutters)
    (Default|OpenShutter _array_element)))

(event EventBeginPlay)

(event Collision|EventActorBeginOverlap
  (params (OtherActor :type Actor%20Object%20Reference)))

(event EventTick
  (params (DeltaSeconds :type Float%20%28single-precision%29)))

(fn ConstructionScript
  (bind _spawnradius (Variables|Default|GetSpawnRadius))
  (Variables|Default|SetQueuePositions (Utilities|Array|MakeArray (Variables|Default|GetArrow)))
  (for _index (range 2 (Variables|Default|GetQueueLength))
    (bind _returnvalue (AddComponent|AddArrowComponent false (Math|Transform|MakeTransform (Math|Vector|MakeVector 0.0 (* (- _index 1) (Variables|Default|GetQueueSpacing)) 0.0) "0.000000,-90.000000, 0" "1,1,1")))
    (Utilities|Array|Add (Variables|Default|GetQueuePositions) _returnvalue)
    (Transformation|SetWorldLocation (Variables|Default|GetBillboard) (Variables|Default|GetExitLocation) false false)
    (Transformation|SetWorldLocation _spawnradius (Variables|Default|GetCustomerSpawnLocation) false false)
    (Components|Sphere|SetSphereRadius _spawnradius (Variables|Default|GetCustomerSpawnRadius) true)))

(fn GetSpawnLocation
  (return (+ (Variables|Default|GetCustomerSpawnLocation) (* (Math|Vector|MakeVector (Math|Random|RandomFloatinRange -1.0 1.0) (Math|Random|RandomFloatinRange -1.0 1.0) 0.0) (Math|Random|RandomFloatinRange 0.0 (Variables|Default|GetCustomerSpawnRadius))))))