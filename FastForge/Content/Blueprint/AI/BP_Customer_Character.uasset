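; AI customer character that orders an item at a counter and pays coins when served.
; ShowOrder picks an item from the Items data table by cumulative ChanceOfOrder weighting, displays it in a widget and listens for counter placements.
; After a grace period, a looping timer decays the coin multiplier.
; A matching item pays between MinSelling and MaxSelling by that multiplier, then the customer heads to the queue exit and is destroyed.
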(event Custom|ShowOrder
  (params (Counter :type BP%20Counter%20Object%20Reference))
  (Variables|Default|SetForward (Math|Vector|GetForwardVector (Variables|Default|GetArrow1)))
  (EventDispatchers|BindEventtoOnObjectPlaced Counter (delegate Custom|checkCounterItem))
  (Rendering|SetVisibility (Variables|Default|GetWidget) true false)
  (bind _orders (CallFunction|GetOrders))
  ;[1 1 1] Get random item ID instead of whole structure
  (bind _item (CallFunction|RandomItem _orders))
  (bind _output_get (Variables|Default|SetOrder _item))
  (bind _returnvalue (Utilities|GetDataTableRow (Variables|Default|GetItems) (Utilities|String|StringToName _output_get))
    (:then
      (bind _returnvalue_2 (UserInterface|CreateWidget "/Game/Blueprint/UI/UI_Order.UI_Order_C" 0 (.ItemName (Utilities|Struct|BreaksItemData _returnvalue))))
      (UserInterface|SetWidget (Variables|Default|GetWidget) _returnvalue_2)
      (Utilities|Time|SetTimerbyEvent (delegate Custom|Patience) 1e+01))))

(event Custom|checkCounterItem
  (params (ItemID :type String) (Counter :type BP%20Counter%20Object%20Reference))
  (if (Utilities|Enum|Equal(Enum) ItemID (Variables|Default|GetOrder))
    (Utilities|Time|ClearandInvalidateTimerbyHandle (Variables|Default|GetPatienceTimer))
    (Default|RemoveObject Counter false)
    (Effects|SpawnEmitteratLocation "/Game/Blueprint/ProgrammerArt/PS_CoinExplode.PS_CoinExplode" (Transformation|GetActorLocation Counter))
    (bind _returnvalue (Utilities|GetDataTableRow (Variables|Default|GetItems) (Utilities|String|StringToName (Variables|Default|GetOrder)))
      (:then
        (bind _controller (Class|IGamemode|GetPlayerController(Message) (Game|GetGameMode)))
        (Class|IController|ModifyCoins(Message) _controller (Math|Float|Round (Math|Float|Lerp (Math|Conversions|ToFloat(Integer) (.MinSelling (Utilities|Struct|BreaksItemData _returnvalue))) (Math|Conversions|ToFloat(Integer) (.MaxSelling (Utilities|Struct|BreaksItemData _returnvalue))) (Variables|Default|GetCoinMultiplier))))
        (Class|IController|TryCharacterMove(Message) (Pawn|GetController) (Variables|/Game/Blueprint/AI/BP_Queue.BP_Queue_C|GetExitLocation (Variables|Default|GetQueue)))
        (Utilities|FlowControl|Delay 2.0)
        (Actor|DestroyActor)))))

(event Custom|Patience
  (bind _returnvalue (Utilities|Time|SetTimerbyEvent (delegate Custom|DeductCoin) 1.0 true))
  (Variables|Default|SetPatienceTimer _returnvalue))

(event Custom|DeductCoin
  (Variables|Default|SetCoinMultiplier (Math|Float|Clamp(Float) (- (Variables|Default|GetCoinMultiplier) 0.05))))

(fn ConstructionScript)

(fn GetOrders
  (bind _items (Variables|Default|GetItems))
  (bind _outrownames (DataTable|GetDataTableRowNames _items))
  (for _array_element _outrownames
    (bind _returnvalue (Utilities|GetDataTableRow _items _array_element)
      (:then
        (if (> (.ChanceOfOrder (Utilities|Struct|BreaksItemData _returnvalue)) 0.0)
          (Utilities|Map|Add (LocalVariables|GetOrderList) (Utilities|String|ToString(Name) _array_element) (.ChanceOfOrder (Utilities|Struct|BreaksItemData _returnvalue)))))))
  (return (LocalVariables|GetOrderList)))

(fn RandomItem
  (params (Items :type Map%20of%20Strings%20to%20Float%20%28single-precision%29s))
  (bind _output_get (LocalVariables|SetItemMap Items))
  (LocalVariables|SetRandomVal (Math|Random|RandomFloatinRange 0.0 1.0))
  (bind _keys (Utilities|Map|Keys _output_get))
  (for _array_element _keys
    (if (< (LocalVariables|GetRandomVal) (+ (.Value (Utilities|Map|Find (LocalVariables|GetItemMap) _array_element)) (LocalVariables|GetCumulativePercent)))
      (return _array_element)
      (else
        (LocalVariables|SetCumulativePercent (+ (.Value (Utilities|Map|Find (LocalVariables|GetItemMap) _array_element)) (LocalVariables|GetCumulativePercent)))))))