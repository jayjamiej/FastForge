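; Ambient pedestrian spawner that continuously spawns BP_Ambient actors from two arrow markers.
; A short delay after BeginPlay starts SpawnCharacter, which re-arms its own one-shot timer with a random interval after each spawn.
; Each spawn randomly picks between the arrows for its transform and offsets sideways along the right vector within SpawnRadius.
; The construction script positions Arrow1 at SpawnDistance along local X.
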(event Custom|SpawnCharacter
  (bind _returnvalue (Math|Random|RandomBool))
  (bind _arrow (Variables|Default|GetArrow))
  (bind _spawnradius (Variables|Default|GetSpawnRadius))
  (bind _arrow1 (Variables|Default|GetArrow1))
  (bind _returnvalue_2 (select _returnvalue _arrow1 _arrow))
  (bind _returnvalue_3 (Transformation|GetWorldTransform _returnvalue_2))
  (Game|SpawnActorfromClass "/Game/Blueprint/AI/BP_Ambient.BP_Ambient_C" (Math|Transform|MakeTransform (+ (.location _returnvalue_3) (* (Math|Vector|GetRightVector _returnvalue_2) (Math|Random|RandomFloatinRange (- 0.0 _spawnradius) _spawnradius))) (.rotation _returnvalue_3) (.scale _returnvalue_3)) "Undefined" 0 0)
  (Utilities|Time|SetTimerbyEvent (delegate Custom|SpawnCharacter) (Math|Random|RandomFloatinRange 1.0 5.0)))

(event EventBeginPlay
  (Utilities|Time|SetTimerbyEvent (delegate Custom|SpawnCharacter) 2.0))

(fn ConstructionScript
  (Transformation|SetRelativeLocation (Variables|Default|GetArrow1) (Math|Vector|MakeVector (Variables|Default|GetSpawnDistance) 0.0 0.0) false false))