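; Furnace bellows machine that keeps its linked Furnace cooking while heat charge lasts.
; Pumping with the player in range refills charge, resumes cooking, animates the bellows by timeline and starts a looping timer that drains charge, stopping the furnace at zero.
; A progress-button widget shows charge and handles interaction, while a plane and spotlight appear when charge runs low.
; The construction script traces down to ground the plane, which anchors player movement to the bellows.
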(event OnComponentBeginOverlap(Sphere)
  (params (OverlappedComponent :type Primitive%20Component%20Object%20Reference) (OtherActor :type Actor%20Object%20Reference) (OtherComp :type Primitive%20Component%20Object%20Reference) (OtherBodyIndex :type Integer) (bFromSweep :type Boolean) (SweepResult :type Hit%20Result%20Structure%20%28by%20ref%29))
  (bind _scheme (Class|IGameInstance|GetControllerScheme(Message) (Game|GetGameInstance)))
  (switch Utilities|FlowControl|Switch|SwitchoneControllerScheme _scheme
    (:NewEnumerator1
      _)
    (:NewEnumerator2
      _))
  (Class|IUI|ShowInteraction(Message) (UserInterface|GetUserWidgetObject (Variables|Default|GetWidget))))

(event OnComponentEndOverlap(Sphere)
  (params (OverlappedComponent :type Primitive%20Component%20Object%20Reference) (OtherActor :type Actor%20Object%20Reference) (OtherComp :type Primitive%20Component%20Object%20Reference) (OtherBodyIndex :type Integer))
  (bind _scheme (Class|IGameInstance|GetControllerScheme(Message) (Game|GetGameInstance)))
  (switch Utilities|FlowControl|Switch|SwitchoneControllerScheme _scheme
    (:NewEnumerator1
      _)
    (:NewEnumerator2
      _))
  (Class|IUI|HideInteraction(Message) (UserInterface|GetUserWidgetObject (Variables|Default|GetWidget))))

(event Custom|MoveToBellows
  ;[1 1 1] Moves within range of the bellows
  (bind _controller (Class|IGamemode|GetPlayerController(Message) (Game|GetGameMode)))
  (bind _outlocation (CallFunction|ApplyRadialOffset (Pawn|GetControlledPawn _controller) (Transformation|GetWorldLocation (Variables|Default|GetPlane)) 5e+01))
  (Class|IController|TryCharacterMove(Message) _controller _outlocation))

(event Custom|PumpBellows
  ;[1 1 1] Pumps the bellows, lighting the furnace and restarting the extinguish countdown
  (bind _controller (Class|IGamemode|GetPlayerController(Message) (Game|GetGameMode)))
  (if (Collision|IsOverlappingActor (Variables|Default|GetSphere) (Pawn|GetControlledPawn _controller) :!class /Script/Engine.PrimitiveComponent)
    (bind _output_get (Variables|Default|SetCharge 1.0))
    (Default|UpdatePercentage (Variables|Default|GetHeatBar) _output_get)
    (Default|ResumeCook (Variables|Default|GetFurnace))
    (CallFunction|StartExtinguish)
    (CallFunction|PlayAnimation)))

(event Custom|ReduceHeat
  ;[1 1 1] Counting down to extinguish the furnace
  (bind _output_get (Variables|Default|SetCharge (- (Variables|Default|GetCharge) (/ (Variables|Default|GetPercentPerSecond) 1e+02))))
  (Default|UpdatePercentage (Variables|Default|GetHeatBar) _output_get)
  (if (<= _output_get 0.0)
    (Default|StopCook (Variables|Default|GetFurnace))
    (Utilities|Time|ClearandInvalidateTimerbyHandle (Variables|Default|GetTimer))
    (else
      (Rendering|SetVisibility (Variables|Default|GetPlane) (< _output_get 0.25) false)
      (Rendering|SetVisibility (Variables|Default|GetSpotLight) (< _output_get 0.25) false))))

(event Custom|StartExtinguish
  ;[1 1 1] Counting down to extinguish the furnace
  (bind _returnvalue (Utilities|Time|SetTimerbyEvent (delegate Custom|ReduceHeat) 0.1 true))
  (Variables|Default|SetTimer _returnvalue))

(event Custom|PlayAnimation
  (bind _alpha (Timeline|Pump PlayFromStart)
    (:Update
      (Transformation|SetRelativeScale3D (Variables|Default|GetTemp_Bellows_Bag) (Math|Vector|MakeVector 1.0 1.0 (Math|Float|Lerp 1.0 0.25 _alpha)))
      (Transformation|SetRelativeRotation (Variables|Default|GetTemp_Bellows_WoodPlate) (Math|Rotator|MakeRotator 0.0 (Math|Float|Lerp 0.0 12.0 _alpha) 0.0) false false)
      (Transformation|SetRelativeRotation (Variables|Default|GetTemp_Bellows_WoodPlate1) (Math|Rotator|MakeRotator 1.8e+02 (Math|Float|Lerp 0.0 -12.0 _alpha) 0.0) false false))))

(event EventBeginPlay
  (bind _furnace (Variables|Default|GetFurnace))
  ;[1 1 1] Init chain
  (bind _returnvalue (UserInterface|CreateWidget "/Game/Blueprint/UI/UI_ProgressButton.UI_ProgressButton_C"))
  (bind _output_get (Variables|Default|SetHeatBar _returnvalue))
  (UserInterface|SetWidget (Variables|Default|GetWidget) _output_get)
  (EventDispatchers|BindEventtoOnHover _output_get (EventDispatchers|CreateEvent :!event Custom|MoveToBellows))
  (EventDispatchers|BindEventtoOnClicked _output_get (EventDispatchers|CreateEvent :!event Custom|PumpBellows))
  (Utilities|IsValid _furnace
    (:Is%20Valid
      (Default|StopCook _furnace))))

(event EventInteract
  (params (InteractIndex :type Integer) (Interactor :type Actor%20Object%20Reference))
  (if (Collision|IsOverlappingActor (Variables|Default|GetSphere) Interactor :!class /Script/Engine.PrimitiveComponent)
    (Class|IUI|KeyInput(Message) (UserInterface|GetUserWidgetObject (Variables|Default|GetWidget)) InteractIndex)))

(fn ConstructionScript
  (bind _returnvalue (Transformation|GetActorLocation))
  (bind _plane (Variables|Default|GetPlane))
  (bind _returnvalue_2 (Transformation|GetWorldLocation _plane))
  (bind _returnvalue_3 (Math|Vector|MakeVector (.x _returnvalue_2) (.y _returnvalue_2) (.z _returnvalue)))
  (bind (_outhit _returnvalue_4) (Collision|LineTraceByChannel (+ _returnvalue_3 "0, 0,100.000000") (- _returnvalue_3 "0, 0,500.000000") "TraceTypeQuery1" false 0 "None"))
  (if _returnvalue_4
    (Transformation|SetWorldLocation (Variables|Default|GetPlane) (+ (.Location (Collision|BreakHitResult _outhit)) "0, 0,5.000000") false false)))

(fn GetMachineType
  (return "NewEnumerator8"))

(fn IsPlayerOverlappingCollision
  (return false))