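; BP_MatInputMachine is a cooking machine that turns ingredients from the player's inventory into a chosen item.
; It filters the recipe DataTable by machine type, then matches held items on menu open, preferring two-input recipes, to populate the options.
; Selection consumes the inputs, starts a progress bar and upgrade-scaled finish time, and can lock the player in place.
; ResetOptions hands over the finished item and unlocks the player.
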(event Custom|CookingDone
  ;[1 1 1] Cooking
  (Variables|Cook|SetIsCooking false)
  (Default|SetCentreIcon (Variables|Default|GetMenu) "/Game/Blueprint/UI/T_SelectIcon.T_SelectIcon" false))

(event Custom|LockPlayer
  (params (Locked :type Boolean))
  (bind _arrow_0 (Variables|Default|GetArrow_0))
  (bind _returnvalue (Transformation|GetWorldTransform _arrow_0))
  ;[1 1 1] Locks the player into a specific location and rotation
  (if Locked
    (bind _controller (Class|IGamemode|GetPlayerController(Message) (Game|GetGameMode)))
    (Transformation|SetActorTransform (Pawn|GetControlledPawn _controller) (Math|Transform|MakeTransform (Math|Vector|MakeVector (.x (.location _returnvalue)) (.y (.location _returnvalue)) (.z (Transformation|GetActorLocation (Pawn|GetControlledPawn _controller)))) (.rotation _returnvalue) "1,1,1")))
  (Class|IController|LockPlayerMovement(Message) _controller Locked))

(event EventBeginPlay
  ;[1 1 1] Init
  (|CallParentFunction)
  (bind _outrownames (DataTable|GetDataTableRowNames (Variables|Recipe|GetRecipes)))
  ;;[1 1 1] Filters recipes for the machine type
  (for _array_element _outrownames
    (bind _returnvalue (Utilities|GetDataTableRow (Variables|Recipe|GetRecipes) _array_element)
      (:then
        (if (Utilities|Enum|Equal(Enum) (Utilities|Struct|BreaksRecipes _returnvalue) (Variables|Default|GetMachineType))
          (Utilities|Array|Add (Variables|Recipe|GetMachineRecipes) _returnvalue))))))

(event EventOptionsMenuOpened
  ;[1 1 1] Gets the players inventory and finds the correct recipes to show
  (|CallParentFunction)
  (bind _controller (Class|IGamemode|GetPlayerController(Message) (Game|GetGameMode)))
  (bind _items (Class|IController|GetInventory(Message) _controller))
  (bind (_index _returninputs) (Recipe|FindRecipeIndex _items))
  (Variables|Default|SetCanMenuOpen (!= _index -1))
  (Variables|Recipe|SetInputs _returninputs)
  (Variables|Recipe|SetRecipeIndex _index)
  (bind _keys (Utilities|Map|Keys (Utilities|Struct|BreaksRecipes (Utilities|Array|Get(acopy) (Variables|Recipe|GetMachineRecipes) _index))))
  (bind _options (Recipe|RecipetoNameArray _keys))
  (Default|SetDefaultOptions (Variables|Default|GetMenu) _options))

(event EventOptionSelected
  (params (Option :type String))
  ;[1 1 1] Cooking
  (bind _controller (Class|IGamemode|GetPlayerController(Message) (Game|GetGameMode)))
  (Utilities|CanCookNewRecipe _controller
    (:True
      (bind _controller_2 (Class|IGamemode|GetPlayerController(Message) (Game|GetGameMode)))
      (for (_array_element _array_index) (Variables|Recipe|GetInputs)
        ;;[1 1 1] Checks that the player has the correct items and removes them
        (if (Utilities|Enum|NotEqual(Enum) _array_element "")
          (bind _success (Class|IController|RemoveItem(Message) _controller_2 _array_element true))
          (if _success
            (if (and (Math|Boolean|Equal(Boolean) (Variables|Recipe|GetRecipeComplete) false) (== _array_index 1))
              (Variables|Recipe|SetRecipeComplete false)
              (else
                (Variables|Recipe|SetRecipeComplete true)))
            (else
              (Variables|Recipe|SetRecipeComplete false)))))
      ;;[1 1 1] If all the required ingredients have been removed, it will begin cooking
      (if (Variables|Recipe|GetRecipeComplete)
        (bind _output_get (Variables|Default|SetResult (.Value (Utilities|Map|Find (Variables|Default|GetOptionNameToID) Option))))
        (bind _returnvalue (UserInterface|CreateWidget "/Game/Blueprint/UI/UI_ProgressBar.UI_ProgressBar_C" 0 (.Value (Utilities|Map|Find (Utilities|Struct|BreaksRecipes (Utilities|Array|Get(acopy) (Variables|Recipe|GetMachineRecipes) (Variables|Recipe|GetRecipeIndex))) _output_get))))
        (EventDispatchers|BindEventtoOnTimeComplete _returnvalue (delegate Custom|CookingDone))
        (Variables|Default|SetProgress _returnvalue)
        (UserInterface|SetWidget (Variables|Default|GetWidget) _returnvalue)
        (Variables|Cook|SetIsCooking true)
        (Variables|Cook|SetCookFinishTime (Cook|CalculateCookTime (.Value (Utilities|Map|Find (Utilities|Struct|BreaksRecipes (Utilities|Array|Get(acopy) (Variables|Recipe|GetMachineRecipes) (Variables|Recipe|GetRecipeIndex))) _output_get))))
        (Variables|Default|SetCanMenuOpen false)
        ;;[1 1 1] Locks the player into postion if an animation is required
        (if (Variables|Cook|GetLockPlayerDuringCook)
          (CallFunction|LockPlayer true))))))

(event EventResetOptions
  ;[1 1 1] If the recipe has finished cooking, add the recipe to the player's inventory
  (if (Utilities|Enum|NotEqual(Enum) (Variables|Default|GetResult) "")
    (if (>= (Utilities|Time|GetTimeSeconds) (Variables|Cook|GetCookFinishTime))
      (bind _success (CallFunction|GiveItemtoPlayer (Variables|Default|GetResult)))
      (if _success
        (UserInterface|SetWidget (Variables|Default|GetWidget) 0)
        (Variables|Default|SetCanMenuOpen true)
        (CallFunction|LockPlayer false)
        (Default|CallOnItemTaken (Variables|Default|GetResult))
        (Variables|Default|SetResult "")
        (bind _scheme (Class|IGameInstance|GetControllerScheme(Message) (Game|GetGameInstance)))
        (Default|SetCentreIcon (Variables|Default|GetMenu) (Utilities|Select :Index _scheme :NewEnumerator0 "/Game/Blueprint/UI/T_SelectIcon.T_SelectIcon" :NewEnumerator1 "/Game/SourcedContent/MappingIcons/E_Key_Dark.E_Key_Dark" :NewEnumerator2 "/Game/SourcedContent/MappingIcons/XboxOne_Left_Stick_Click.XboxOne_Left_Stick_Click") true)))
    (else
      (|CallParentFunction))))

(fn ConstructionScript
  (|CallParentFunction))

(fn FindRecipeIndex
  (params (Inventory :type Array%20of%20Strings))
  (LocalVariables|SetPlayerInventory Inventory)
  (for (_array_element _array_index) (Variables|Recipe|GetMachineRecipes)
    (LocalVariables|SetCurrentIndex _array_index)
    (LocalVariables|SetInput_Local (Utilities|Array|MakeArray (.InputItem_1 (Utilities|Struct|BreaksRecipes _array_element)) (.InputItem_2 (Utilities|Struct|BreaksRecipes _array_element))))
    (if (or (Utilities|Enum|Equal(Enum) (.InputItem_1 (Utilities|Struct|BreaksRecipes _array_element)) (Utilities|Array|Get(acopy) Inventory)) (Utilities|Enum|Equal(Enum) (.InputItem_1 (Utilities|Struct|BreaksRecipes _array_element)) (Utilities|Array|Get(acopy) Inventory 1)))
      (if (Utilities|Enum|Equal(Enum) (Utilities|Array|Get(acopy) (LocalVariables|GetInput_Local) 1) "")
        (if (not (LocalVariables|GetFoundDualInput))
          (LocalVariables|SetReturnIndex (LocalVariables|GetCurrentIndex)))
        (elif (Utilities|Enum|Equal(Enum) (.InputItem_1 (Utilities|Struct|BreaksRecipes _array_element)) (Utilities|Array|Get(acopy) Inventory))
          (if (Utilities|Enum|Equal(Enum) (Utilities|Array|Get(acopy) (LocalVariables|GetPlayerInventory) 1) (Utilities|Array|Get(acopy) (LocalVariables|GetInput_Local) 1))
            (LocalVariables|SetReturnIndex (LocalVariables|GetCurrentIndex) :!label _label)
            (LocalVariables|SetFoundDualInput true))
          (elif (Utilities|Enum|Equal(Enum) (Utilities|Array|Get(acopy) (LocalVariables|GetPlayerInventory)) (Utilities|Array|Get(acopy) (LocalVariables|GetInput_Local) 1))
            (goto _label))))))
  (return (LocalVariables|GetReturnIndex) (Utilities|Array|MakeArray (.InputItem_1 (Utilities|Struct|BreaksRecipes (Utilities|Array|Get(acopy) (Variables|Recipe|GetMachineRecipes) (LocalVariables|GetReturnIndex)))) (.InputItem_2 (Utilities|Struct|BreaksRecipes (Utilities|Array|Get(acopy) (Variables|Recipe|GetMachineRecipes) (LocalVariables|GetReturnIndex)))))))

(fn RecipetoNameArray
  (params (IDs :type Array%20of%20Strings))
  (bind _items (LocalVariables|GetItems))
  (for _index (range 0 (Utilities|Array|LastIndex IDs))
    (bind _returnvalue (Utilities|GetDataTableRow (Variables|Default|GetItemData) (Utilities|String|StringToName (Utilities|Array|Get(acopy) IDs _index)))
      (:then
        (Utilities|Array|Add _items (Utilities|Struct|MakesMachineOption (.ItemName (Utilities|Struct|BreaksItemData _returnvalue)) (.ItemIcon (Utilities|Struct|BreaksItemData _returnvalue)) (.ItemCost (Utilities|Struct|BreaksItemData _returnvalue)))))
      (:RowNotFound
        (Utilities|Array|Add _items (Utilities|Struct|MakesMachineOption "None" 0 0)))))
  (for _index_2 (range (Utilities|Array|LastIndex (LocalVariables|GetItems)) 3)
    (Utilities|Array|Add (LocalVariables|GetItems) (Utilities|Struct|MakesMachineOption "None")))
  (return (LocalVariables|GetItems)))

(fn GetMachineResult
  (return (Variables|Default|GetResult)))

(fn GetMachineCookFinishTime
  (return (Variables|Cook|GetCookFinishTime)))

(fn SetMachineCookFinishTime
  (params (CookFinishTime :type Float%20%28single-precision%29))
  (Variables|Cook|SetCookFinishTime CookFinishTime))

(fn CalculateCookTime
  (params (InTime :type Float%20%28single-precision%29))
  (return (+ (Utilities|Time|GetTimeSeconds) (/ InTime (Variables|Default|GetCurrentUpgradeBoost)))))