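; BP_Furnace is a cooking machine whose crafting only runs while its fire is lit, with option selection passed to the parent only when lit.
; StopCook turns off fire and light, pauses any active job's progress, saves its remaining time and pushes the finish time to a huge sentinel value.
; ResumeCook relights with a one-shot ignition emitter and rebuilds the finish time from the saved remainder.
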(event Custom|StopCook
  (Variables|Default|SetLit false)
  (Components|Activation|Deactivate (Variables|Default|GetFire))
  (Rendering|Components|Light|SetIntensity (Variables|Default|GetPointLight) 0.0)
  (if (Utilities|Enum|NotEqual(Enum) (CallFunction|GetMachineResult) "")
    (Default|SetProgressPaused (Variables|Default|GetProgress) true)
    (Variables|Default|SetRemainingTime (- (CallFunction|GetMachineCookFinishTime) (Utilities|Time|GetTimeSeconds)))
    (CallFunction|SetMachineCookFinishTime 999999995904.0)
    (Variables|Default|SetIsCooking false)))

(event Custom|ResumeCook
  (bind _arrow1 (Variables|Default|GetArrow1))
  (bind _returnvalue (Transformation|GetWorldTransform _arrow1))
  (if (not (Variables|Default|GetLit))
    (Components|Activation|Activate (Variables|Default|GetFire) false)
    (Variables|Default|SetLit true)
    (Rendering|Components|Light|SetIntensity (Variables|Default|GetPointLight) 5e+03)
    (Effects|SpawnEmitteratLocation "/Game/Blueprint/ProgrammerArt/PS_LightFire.PS_LightFire" (.location _returnvalue) (.rotation _returnvalue))
    (if (Utilities|Enum|NotEqual(Enum) (CallFunction|GetMachineResult) "")
      (Default|SetProgressPaused (Variables|Default|GetProgress) false)
      (CallFunction|SetMachineCookFinishTime (+ (Utilities|Time|GetTimeSeconds) (Variables|Default|GetRemainingTime)))
      (Variables|Default|SetIsCooking true)
      (Variables|Default|SetCanCook false))))

(event EventBeginPlay
  (|CallParentFunction) ; This node is disabled and will not be called.\nDrag off pins to build functionality.
)

(event Collision|EventActorBeginOverlap
  (params (OtherActor :type Actor%20Object%20Reference)))

(event EventTick
  (params (DeltaSeconds :type Float%20%28single-precision%29)))

(event EventOptionSelected
  (params (Option :type String))
  (if (Variables|Default|GetLit)
    (|CallParentFunction Option)))

(fn ConstructionScript
  (|CallParentFunction))