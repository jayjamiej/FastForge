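; BP_Storage is a machine with an options menu that sells metal and miscellaneous items to the player for coins.
; On BeginPlay it applies its option override and builds both category lists from the ItemData table.
; Choosing a category swaps the menu options.
; Choosing an item checks coins, inventory space and player proximity, then grants it through controller messages, deducts its cost and plays a craft sound.
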(event Custom|OverrideOptions
  (CallFunction|SetOptions (Variables|Default|GetOptionsOverride)))

(event Custom|GivePlayerItem
  (params (Target :type Object%20Object%20Reference) (ItemID :type String))
  (Class|IController|GiveItem(Message) Target ItemID))

(event EventBeginPlay
  (CallFunction|OverrideOptions)
  (|CallParentFunction)
  (for _array_element (Utilities|Array|MakeArray "Irn" "Gld" "Tin" "Cop")
    (bind _returnvalue (Utilities|GetDataTableRow (Variables|Default|GetItemData) _array_element)
      (:then
        (Utilities|Array|Add (Variables|Default|GetMetalOptions) (Utilities|Struct|MakesMachineOption (.ItemName (Utilities|Struct|BreaksItemData _returnvalue)) (.ItemIcon (Utilities|Struct|BreaksItemData _returnvalue)) (.ItemCost (Utilities|Struct|BreaksItemData _returnvalue)))))))
  (for _array_element_2 (Utilities|Array|MakeArray "Wod" "Flt" "Col" "Gem")
    (bind _returnvalue_2 (Utilities|GetDataTableRow (Variables|Default|GetItemData) _array_element_2)
      (:then
        (Utilities|Array|Add (Variables|Default|GetMiscOptions) (Utilities|Struct|MakesMachineOption (.ItemName (Utilities|Struct|BreaksItemData _returnvalue_2)) (.ItemIcon (Utilities|Struct|BreaksItemData _returnvalue_2)) (.ItemCost (Utilities|Struct|BreaksItemData _returnvalue_2))))))))

(event EventOptionSelected
  (params (Option :type String))
  (bind _menu (Variables|Default|GetMenu))
  (switch string Option
    (:Default
      (bind _controller (Class|IGamemode|GetPlayerController(Message) (Game|GetGameMode)))
      (bind _total (Class|IController|GetPlayerCoins(Message) _controller))
      (bind _value (CallFunction|GetItemValue (Utilities|Text|ToText(String) Option)))
      (if (>= _total _value)
        (bind _isfull (Class|IController|GetInventory(Message) _controller))
        (if (not _isfull)
          (if (Collision|IsOverlappingActor (Variables|Default|GetPlayerRadius) (Pawn|GetControlledPawn _controller) :!class /Script/Engine.PrimitiveComponent)
            (CallFunction|GivePlayerItem _controller (.Value (Utilities|Map|Find (Variables|Default|GetOptionNameToID) Option)))
            (Class|IController|ModifyCoins(Message) _controller (- 0 _value))
            (Audio|PlaySoundatLocation "/Game/Sounds/Workbench/CUE_Craft.CUE_Craft" (Transformation|GetActorLocation) "0, 0, 0" 1.0 1.0 0.0 0 0 0)))))
    (:Metal
      (Default|SetOptions _menu (Variables|Default|GetMetalOptions)))
    (:Misc
      (Default|SetOptions _menu (Variables|Default|GetMiscOptions)))))

(event EventOptionsMenuOpened
  (|CallParentFunction))

(fn ConstructionScript
  (|CallParentFunction))

(fn GetItemValue
  (params (ItemName :type Text))
  (bind _returnvalue (Utilities|GetDataTableRow (Variables|Default|GetItemData) (Utilities|String|StringToName (.Value (Utilities|Map|Find (Variables|Default|GetOptionNameToID) (Utilities|String|ToString(Text) ItemName)))))
    (:then
      (return (.ItemCost (Utilities|Struct|BreaksItemData _returnvalue))))
    (:RowNotFound
      (return 0))))