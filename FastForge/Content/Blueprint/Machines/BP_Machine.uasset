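; Base Blueprint for the blacksmith's machines, with crafting options and coin-bought upgrades, leaving option and cook events as placeholders for child classes.
; A widget component switches between options and upgrade menus, offering upgrades only when affordable.
; Selection moves the player toward a floor-snapped marker, and a sphere overlap gates the options menu and item handouts.
; Each level's upgrade data sets boost, mesh and material, with particles on upgrade.
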(event OnComponentBeginOverlap(PlayerRadius)
  (params (OverlappedComponent :type Primitive%20Component%20Object%20Reference) (OtherActor :type Actor%20Object%20Reference) (OtherComp :type Primitive%20Component%20Object%20Reference) (OtherBodyIndex :type Integer) (bFromSweep :type Boolean) (SweepResult :type Hit%20Result%20Structure%20%28by%20ref%29))
  ;[1 1 1] Overlap checks to make sure the player is in postion to use the machine
  (if (== (Utilities|GetClass OtherActor) "/Game/Blueprint/Player/BP_Blacksmith_Character.BP_Blacksmith_Character_C")
    (if (Variables|Machine|GetMachineSelected)
      (CallFunction|OptionsMenuOpened))))

(event OnComponentEndOverlap(PlayerRadius)
  (params (OverlappedComponent :type Primitive%20Component%20Object%20Reference) (OtherActor :type Actor%20Object%20Reference) (OtherComp :type Primitive%20Component%20Object%20Reference) (OtherBodyIndex :type Integer))
  ;[1 1 1] Overlap checks to make sure the player is in postion to use the machine
  (if (== (Utilities|GetClass OtherActor) "/Game/Blueprint/Player/BP_Blacksmith_Character.BP_Blacksmith_Character_C")
    (Default|PlayerLeftRadius (Variables|Default|GetMenu))))

(event Custom|OptionSelected
  (params (Option :type String))
  ;[1 1 1] Event holders for child classes bound to events in the UI
  (Development|PrintString "Option selected"))

(event Custom|resetOptions
  (bind _menu (Variables|Default|GetMenu))
  ;[1 1 1] UI bound events
  (if (Variables|/Game/Blueprint/UI/UI_MachineOptions.UI_MachineOptions_C|GetOptionsChanged _menu)
    (Default|ResetOptionstoDefault _menu)))

(event Custom|Cook
  (params (Result :type String))
  ;[1 1 1] Event holders for child classes bound to events in the UI
  (Development|PrintString "Cook started"))

(event Custom|OptionsMenuOpened
  ;[1 1 1] UI bound events
  (Variables|Machine|SetMachineSelected true)
  (CallFunction|MoveIntoRadius)
  (bind _controller (Class|IGamemode|GetPlayerController(Message) (Game|GetGameMode)))
  (if (Collision|IsOverlappingActor (Variables|Default|GetPlayerRadius) (Pawn|GetControlledPawn _controller) :!class /Script/Engine.PrimitiveComponent)
    (if (Variables|UI|GetCanMenuOpen)
      (Default|ShowMenu (Variables|Default|GetMenu)))))

(event Custom|MoveIntoRadius
  ;[1 1 1] UI bound events
  ;;[1 1 1] Moves the player to the correct position when the cursor overlaps with the menu
  (bind _controller (Class|IGamemode|GetPlayerController(Message) (Game|GetGameMode)))
  (bind _outlocation (CallFunction|ApplyRadialOffset (Pawn|GetControlledPawn _controller) (Transformation|GetWorldLocation (Variables|Default|GetPlane)) 5e+01))
  (Class|IController|TryCharacterMove(Message) _controller _outlocation)
  (Transformation|SetWorldRotation (Variables|Default|GetArrow) "0, 0, 0" false false))

(event Custom|MenuClose
  ;[1 1 1] Init Chain
  ;;[1 1 1] UI Init
  (Variables|Machine|SetMachineSelected false))

(event Custom|UpgradeMachine
  (bind _level (Variables|UpgradeSystem|GetLevel))
  ;[1 1 1] Upgrade machine from UI input
  (Rendering|SetVisibility (Variables|Default|GetMenuWidget) false false)
  (Math|Integer|IncrementInt _level
    (:%20%20
      (bind _controller (Class|IGamemode|GetPlayerController(Message) (Game|GetGameMode)))
      (Class|IController|ModifyCoins(Message) _controller (- 0 (.upgradecost (.Value (Utilities|Map|Find (Variables|UpgradeSystem|GetUpgrades) _level)))))
      (CallFunction|SetLevel true))))

(event EventBeginPlay
  ;[1 1 1] Init Chain
  (CallFunction|NametoIDSetup)
  ;;[1 1 1] UI Init
  (bind _returnvalue (UserInterface|CreateWidget "/Game/Blueprint/UI/UI_Upgrade.UI_Upgrade_C" 0 self))
  (Variables|UpgradeSystem|SetUpgradeMenu _returnvalue)
  (bind _returnvalue_2 (UserInterface|CreateWidget "/Game/Blueprint/UI/UI_MachineOptions.UI_MachineOptions_C" 0 (Variables|Machine|GetOptions) (Variables|UI|GetShowOptionValues) self))
  (bind _output_get (Variables|Default|SetMenu _returnvalue_2))
  (UserInterface|SetWidget (Variables|Default|GetMenuWidget) _output_get)
  (EventDispatchers|BindEventtoOnOptionSelected (Variables|Default|GetMenu) (EventDispatchers|CreateEvent :!event Custom|OptionSelected))
  (EventDispatchers|BindEventtoOnCenterPressed (Variables|Default|GetMenu) (EventDispatchers|CreateEvent :!event Custom|resetOptions))
  (EventDispatchers|BindEventtoOnOptionsHovered (Variables|Default|GetMenu) (EventDispatchers|CreateEvent :!event Custom|OptionsMenuOpened))
  (EventDispatchers|BindEventtoOnMenuClosed (Variables|Default|GetMenu) (delegate Custom|MenuClose))
  (CallFunction|SetLevel false))

(fn ConstructionScript
  (bind _plane (Variables|Default|GetPlane))
  (bind _returnvalue (Transformation|GetWorldLocation _plane))
  (Components|Sphere|SetSphereRadius (Variables|Default|GetPlayerRadius) (Variables|Machine|GetOperableRadius) true)
  (Transformation|SetRelativeLocation _plane (Math|Vector|MakeVector (Variables|Machine|GetInteractDistance) 0.0 0.0) false false)
  (bind (_outhit _returnvalue_2) (Collision|LineTraceByChannel _returnvalue (- _returnvalue "0, 0,300.000000") "TraceTypeQuery1" false 0 "None"))
  (if _returnvalue_2
    (Transformation|SetWorldLocation (Variables|Default|GetPlane) (+ (.Location (Collision|BreakHitResult _outhit)) "0, 0,2.000000") false false)))

(fn NametoIDSetup
  (bind _outrownames (DataTable|GetDataTableRowNames (Variables|Default|GetItemData)))
  (for _array_element _outrownames
    (bind _returnvalue (Utilities|GetDataTableRow (Variables|Default|GetItemData) _array_element)
      (:then
        (Utilities|Map|Add (Variables|Machine|GetOptionNameToID) (Utilities|String|ToString(Name) (.ItemName (Utilities|Struct|BreaksItemData _returnvalue))) (Utilities|String|ToString(Name) _array_element))))))

(fn SwitchMenuType
  (params (Type :type eMenuType%20Enum :default "NewEnumerator0"))
  (bind _menuwidget (Variables|Default|GetMenuWidget))
  (bind _upgrademenu (Variables|UpgradeSystem|GetUpgradeMenu))
  (bind _level (Variables|UpgradeSystem|GetLevel))
  (bind _upgrades (Variables|UpgradeSystem|GetUpgrades))
  (bind _returnvalue (+ _level 1))
  (bind (_value _returnvalue_2) (Utilities|Map|Find _upgrades _returnvalue))
  (bind _upgradecost (Utilities|Struct|BreaksUpgrade2 _value))
  (switch Utilities|FlowControl|Switch|SwitchoneMenuType Type
    (:NewEnumerator0
      (UserInterface|SetWidget (Variables|Default|GetMenuWidget) (Variables|Default|GetMenu))
      (Rendering|SetVisibility (Variables|Default|GetMenuWidget) true false))
    (:NewEnumerator1
      (bind _controller (Class|IGamemode|GetPlayerController(Message) (Game|GetGameMode)))
      (bind _total (Class|IController|GetPlayerCoins(Message) _controller))
      (if _returnvalue_2
        (if (>= _total _upgradecost)
          (UserInterface|SetWidget _menuwidget _upgrademenu)
          (Default|Update _upgrademenu _upgradecost)
          (else
            (Rendering|SetVisibility _menuwidget false false :!label _label)))
        (else
          (goto _label))))))

(fn ShowPlayerLocation
  (params (bNewVisibility :type Boolean))
  (Rendering|SetVisibility (Variables|Default|GetPlane) bNewVisibility false)
  (Rendering|SetVisibility (Variables|Default|GetSpotLight) bNewVisibility false))

(fn SetOptions
  (params (Options :type Array%20of%20S%20Machine%20Option%20Structures))
  (Variables|Machine|SetOptions Options))

(fn SetLevel
  (params (UseFX :type Boolean))
  (bind _upgrades (Variables|UpgradeSystem|GetUpgrades))
  (bind _level (Variables|UpgradeSystem|GetLevel))
  (bind _staticmesh (Variables|Default|GetStaticMesh))
  (bind _value (Utilities|Map|Find _upgrades _level))
  (Variables|Default|SetCurrentUpgradeBoost (.upgradeboost _value))
  (if UseFX
    (Components|Activation|Activate (Variables|Default|GetPS_Upgrade) false))
  (Utilities|IsValid (.upgrademesh _value)
    (:Is%20Valid
      (Components|StaticMesh|SetStaticMesh _staticmesh (.upgrademesh _value))
      (Utilities|IsValid (.upgradematerial _value)
        (:Is%20Valid
          (Rendering|Material|SetMaterial _staticmesh 0 (.upgradematerial _value)))))))

(fn GiveItemtoPlayer
  (params (ItemID_ToGive :type String))
  (bind _controller (Class|IGamemode|GetPlayerController(Message) (Game|GetGameMode)))
  (if (Collision|IsOverlappingActor (Variables|Default|GetPlayerRadius) (Pawn|GetControlledPawn _controller) :!class /Script/Engine.PrimitiveComponent)
    (bind _success (Class|IController|GiveItem(Message) _controller ItemID_ToGive))
    (return _success)
    (else
      (return false))))

(fn GetMachineType
  (return (Variables|Machine|GetMachineType)))

(fn IsPlayerOverlappingCollision
  (bind _controller (Class|IGamemode|GetPlayerController(Message) (Game|GetGameMode)))
  (return (Collision|IsOverlappingActor (Variables|Default|GetPlayerRadius) (Pawn|GetControlledPawn _controller) :!class /Script/Engine.PrimitiveComponent)))