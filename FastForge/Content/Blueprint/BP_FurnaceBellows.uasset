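; Furnace bellows actor that the player pumps to keep a linked Furnace cooking.
; A progress-button widget shows the charge, and hovering it asks the player controller to move the character to the bellows' Plane.
; Clicking it while the controlled pawn overlaps the Sphere refills the charge and resumes cooking.
; A looping timer drains the charge and stops the Furnace cooking once it is empty.
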(event Custom|MoveToBellows
  (bind _controller (Class|IGamemode|GetPlayerController(Message) (Game|GetGameMode)))
  (Class|IController|TryCharacterMove(Message) _controller (Transformation|GetWorldLocation (Variables|Default|GetPlane))))

(event Custom|PumpBellows
  (bind _controller (Class|IGamemode|GetPlayerController(Message) (Game|GetGameMode)))
  (if (Collision|IsOverlappingActor (Variables|Default|GetSphere) (Pawn|GetControlledPawn _controller) :!class /Script/Engine.PrimitiveComponent)
    (bind _output_get (Variables|Default|SetCharge 1.0))
    (Default|UpdatePercentage (Variables|Default|GetHeatBar) _output_get)
    (Default|ResumeCook (Variables|Default|GetFurnace))))

(event Custom|ReduceHeat
  (bind _output_get (Variables|Default|SetCharge (- (Variables|Default|GetCharge) (/ (Variables|Default|GetPercentPerSecond) 1e+02))))
  (Default|UpdatePercentage (Variables|Default|GetHeatBar) _output_get)
  (if (<= _output_get 0.0)
    (Default|StopCook (Variables|Default|GetFurnace))))

(event EventBeginPlay
  (bind _returnvalue (UserInterface|CreateWidget "/Game/Blueprint/UI_ProgressButton.UI_ProgressButton_C"))
  (bind _output_get (Variables|Default|SetHeatBar _returnvalue))
  (UserInterface|SetWidget (Variables|Default|GetWidget) _output_get)
  (EventDispatchers|BindEventtoOnHover _output_get (delegate Custom|MoveToBellows))
  (EventDispatchers|BindEventtoOnClicked _output_get (delegate Custom|PumpBellows))
  (Utilities|Time|SetTimerbyEvent (delegate Custom|ReduceHeat) 0.1 true))

(fn ConstructionScript)