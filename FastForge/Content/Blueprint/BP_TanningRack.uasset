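; Tanning rack crafting station that turns a chosen recipe option into a timed job, built on a parent station Blueprint.
; GivePlayerItem looks up the craft time in the "Tanner" row of the Recipes table, shows a progress bar widget and blocks the menu.
; ResetOptions hands over the finished item if the player is within radius, clearing the state on success, and defers to the parent when idle.
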(event EventBeginPlay
  (|CallParentFunction) ; This node is disabled and will not be called.\nDrag off pins to build functionality.
)

(event Collision|EventActorBeginOverlap
  (params (OtherActor :type Actor%20Object%20Reference))
  (|CallParentFunction OtherActor) ; This node is disabled and will not be called.\nDrag off pins to build functionality.
)

(event EventTick
  (params (DeltaSeconds :type Float%20%28single-precision%29))
  (|CallParentFunction DeltaSeconds) ; This node is disabled and will not be called.\nDrag off pins to build functionality.
)

(event EventGivePlayerItem
  (params (Target :type Object%20Object%20Reference) (ItemID :type String))
  (bind _output_get (Variables|Default|SetResultID ItemID))
  (bind _returnvalue (Utilities|GetDataTableRow (Variables|Default|GetRecipes) "Tanner")
    (:then
      (bind _returnvalue_2 (UserInterface|CreateWidget "/Game/Blueprint/UI_ProgressBar.UI_ProgressBar_C" 0 (.Value (Utilities|Map|Find (.OptionsAndTime (Utilities|Struct|BreaksRecipes _returnvalue)) _output_get))))
      (UserInterface|SetWidget (Variables|Default|GetWidget) _returnvalue_2)
      (Variables|Default|SetIsCooking true)
      (Variables|Default|SetCookFinishTime (+ (Utilities|Time|GetTimeSeconds) 1.0))
      (Variables|Default|SetCanMenuOpen false))))

(event EventResetOptions
  (if (Variables|Default|GetIsCooking)
    (if (>= (Utilities|Time|GetTimeSeconds) (Variables|Default|GetCookFinishTime))
      (bind _controller (Class|IGamemode|GetPlayerController(Message) (Game|GetGameMode)))
      (if (Collision|IsOverlappingActor (Variables|Default|GetPlayerRadius) (Pawn|GetControlledPawn _controller) :!class /Script/Engine.PrimitiveComponent)
        (bind _success (Class|IController|GiveItem(Message) _controller (Variables|Default|GetResultID)))
        (if _success
          (UserInterface|SetWidget (Variables|Default|GetWidget) 0)
          (Variables|Default|SetIsCooking false)
          (Variables|Default|SetCanMenuOpen true))))
    (else
      (|CallParentFunction))))

(fn ConstructionScript
  (|CallParentFunction))