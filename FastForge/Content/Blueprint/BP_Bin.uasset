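; BP_Bin is an interactable bin that stores up to four items from the player's inventory and hands them back through an options menu.
; ResetOptions moves the player's last item into the bin if space remains, via controller messages obtained through the GameMode.
; GetInventoryNames resolves four slots through the ItemData table, showing "None" for missing rows.
; Selecting an option gives that item back, removing it and refreshing the menu on success.
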(event EventResetOptions
  (if (< (Utilities|Array|Length (Variables|Default|GetInventory)) 4)
    (bind _controller (Class|IGamemode|GetPlayerController(Message) (Game|GetGameMode)))
    (bind _items (Class|IController|GetInventory(Message) _controller))
    (Utilities|Array|Add (Variables|Default|GetInventory) (Utilities|Array|Get(acopy) _items (Utilities|Array|LastIndex _items)))
    (bind _names (CallFunction|GetInventoryNames))
    (Default|SetOptions (Variables|Default|GetMenu) _names)
    (Class|IController|RemoveItem(Message) _controller (Utilities|Array|Get(acopy) _items (Utilities|Array|LastIndex _items)))))

(event EventBeginPlay
  (|CallParentFunction))

(event EventOptionsMenuOpened
  (bind _names (CallFunction|GetInventoryNames))
  (Default|SetDefaultOptions (Variables|Default|GetMenu) _names)
  (|CallParentFunction))

(event EventOptionSelected
  (params (Option :type String))
  (bind _optionnametoid (Variables|Default|GetOptionNameToID))
  (bind _inventory (Variables|Default|GetInventory))
  (bind _value (Utilities|Map|Find _optionnametoid Option))
  (bind _controller (Class|IGamemode|GetPlayerController(Message) (Game|GetGameMode)))
  (bind _success (Class|IController|GiveItem(Message) _controller _value))
  (if _success
    (Utilities|Array|RemoveIndex _inventory (Utilities|Array|FindItem _inventory _value))
    (bind _names (CallFunction|GetInventoryNames))
    (Default|SetDefaultOptions (Variables|Default|GetMenu) _names)))

(fn ConstructionScript)

(fn GetInventoryNames
  (bind _items (LocalVariables|GetItems))
  (for _index (range 0 3)
    (bind _returnvalue (Utilities|GetDataTableRow (Variables|Default|GetItemData) (Utilities|String|StringToName (Utilities|Array|Get(acopy) (Variables|Default|GetInventory) _index)))
      (:then
        (Utilities|Array|Add _items (.ItemName (Utilities|Struct|BreaksItemData _returnvalue))))
      (:RowNotFound
        (Utilities|Array|Add _items "None"))))
  (return (LocalVariables|GetItems)))