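; BP_Workbench is a workbench Blueprint that extends a parent class with a player-locking event.
; Its LockPlayer override calls the parent, then sends an animation state message through the player controller message object obtained from the game mode.
; The Locked flag selects between two animation states.
; All other events are disabled stubs, and construction only calls the parent.
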(event EventBeginPlay
  (|CallParentFunction) ; This node is disabled and will not be called.\nDrag off pins to build functionality.
)

(event Collision|EventActorBeginOverlap
  (params (OtherActor :type Actor%20Object%20Reference))
  (|CallParentFunction OtherActor) ; This node is disabled and will not be called.\nDrag off pins to build functionality.
)

(event EventTick
  (params (DeltaSeconds :type Float%20%28single-precision%29))
  (|CallParentFunction DeltaSeconds) ; This node is disabled and will not be called.\nDrag off pins to build functionality.
)

(event EventLockPlayer
  (params (Locked :type Boolean))
  (|CallParentFunction Locked)
  (bind _controller (Class|IGamemode|GetPlayerController(Message) (Game|GetGameMode)))
  (Class|IController|SetAnimationState(Message) _controller (select Locked "NewEnumerator1" "NewEnumerator0")))

(fn ConstructionScript
  (|CallParentFunction))