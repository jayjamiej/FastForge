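; iController is an interface-style set of function stubs for controllers, covering inventory, coins, movement and animation state.
; It declares calls to query the inventory, give or remove items by ID, and read or modify player coins.
; Further calls attempt a character move to a location, get or set the animation state, and lock player movement.
; The functions hold no logic, returning only default values or nothing, so any behavior comes from implementers.
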(fn GetInventory
  (return 0 false))

(fn GiveItem
  (params (ItemID :type String))
  (return false))

(fn ModifyCoins
  (params (In :type Integer))
  (return 0))

(fn GetPlayerCoins
  (return 0))

(fn TryCharacterMove
  (params (Location :type Vector))
  (return false))

(fn RemoveItem
  (params (ItemID :type String))
  (return false))

(fn GetAnimState
  (return "NewEnumerator0"))

(fn SetAnimationState
  (params (State :type eAnimState%20Enum :default "NewEnumerator0")))

(fn LockPlayerMovement
  (params (Locked :type Boolean)))